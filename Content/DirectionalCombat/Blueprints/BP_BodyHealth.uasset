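; BP_BodyHealth is an unfinished body health component that listens for point damage on its owning actor.
; For skeletal mesh hits, it fetches the weapon message from the damage causer through a hard-coded true branch.
; The unreachable false branch detaches the hit mesh from its master pose, then ragdolls it with an impulse.
; A damage calculation using blunt, slash and pierce resistances is left unconnected.
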(event `self.ReceiveBeginPlay`
  (add `Actor.OnTakePointDamage` (`self.GetOwner`) (delegate `OnTakePointDamage_Event_0`)))

(event `OnTakePointDamage_Event_0`
  (params (DamagedActor :type "Actor Object Reference") (Damage :type "Float (double-precision)") (InstigatedBy :type "Controller Object Reference") (HitLocation :type "Vector Structure") (FHitComponent :type "PrimitiveComponent Object Reference") (BoneName :type Name) (ShotFromDirection :type "Vector Structure") (DamageType :type "DamageType Object Reference") (DamageCauser :type "Actor Object Reference"))
  (bind _asskeletal_mesh_component (cast `SkeletalMeshComponent` FHitComponent))
  (if true
    (bind _curweapon (message `/Game/DirectionalCombat/Blueprints/Interfaces/I_Combat.GetWeapon` DamageCauser))
    (else
      (`SkinnedMeshComponent.SetLeaderPoseComponent` _asskeletal_mesh_component null false)
      (`KismetSystemLibrary.Delay` 0.2)
      (`PrimitiveComponent.SetSimulatePhysics` _asskeletal_mesh_component true)
      (`PrimitiveComponent.AddImpulse` _asskeletal_mesh_component HitLocation "None" true))))