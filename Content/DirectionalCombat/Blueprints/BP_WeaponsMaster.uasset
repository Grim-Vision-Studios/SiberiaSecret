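; BP_WeaponsMaster holds the list of weapon definitions and spawns dropped weapons for the directional combat system.
; Its construction script fills the Weapons array with unique rows from DT_Weapons, which SetCurWeapon and SetWeapon return by index.
; DropWeapon spawns a BP_WeaponActor at a given transform and passes it the weapon through SpawnWeaponMessage.
; EditWeapon and GetWeapon are empty, and GetCharacterStatus returns only default values.
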(event `/Game/DirectionalCombat/Blueprints/Interfaces/I_Combat.Drop Weapon`
  (params (CurrWeapon :type "/Game/DirectionalCombat/Blueprints/Data/S_Weapon Structure") (Location :type "Vector Structure") (Rotation :type "Rotator Structure"))
  (set `self.CurrWeapon` CurrWeapon)
  (bind _returnvalue (`|SpawnActorFromClass` "/Game/DirectionalCombat/Blueprints/BP_WeaponActor.BP_WeaponActor_C" (`KismetMathLibrary.MakeTransform` Location Rotation) "Undefined" "OverrideRootScale" null null))
  (message `/Game/DirectionalCombat/Blueprints/Interfaces/I_Intereactable.SpawnWeapon` _returnvalue (`self.CurrWeapon`)))

(fn `Edit Weapon`
  (params (CurrWeapon :type "/Game/DirectionalCombat/Blueprints/Data/S_Weapon Structure") (EditType :type "/Game/DirectionalCombat/Blueprints/Data/E_Upgrades Enum" :default "NewEnumerator0"))
  (returns (UpgradedWeapon :type "/Game/DirectionalCombat/Blueprints/Data/S_Weapon Structure"))
  (return))

(fn `GetCharacterStatus`
  (returns (HasWeapon :type Boolean) (IsAttacking :type Boolean) (IsBlocking :type Boolean) (IsKicking :type Boolean) (isPrepared :type Boolean) (AimDirection :type "/Game/DirectionalCombat/Blueprints/Data/E_AimDirection Enum"))
  (return false false false false false "NewEnumerator0"))

(fn `GetWeapon`
  (returns (CurWeapon :type "/Game/DirectionalCombat/Blueprints/Data/S_Weapon Structure"))
  (return))

(fn `SetCurWeapon`
  (params (Index :type Integer))
  (returns (Output :type "/Game/DirectionalCombat/Blueprints/Data/S_Weapon Structure"))
  (return (`|GetArrayItem` (`self.Weapons`) Index)))

(fn `SetWeapon`
  (params (WeaponIndex :type Integer))
  (returns (NewCurrWeapon :type "/Game/DirectionalCombat/Blueprints/Data/S_Weapon Structure"))
  (return (`|GetArrayItem` (`self.Weapons`) WeaponIndex)))

(fn `UserConstructionScript`
  (bind _outrownames (`DataTableFunctionLibrary.GetDataTableRowNames` "/Game/DirectionalCombat/Blueprints/Data/DataTables/DT_Weapons.DT_Weapons"))
  (for _array_element _outrownames
    (bind _returnvalue (`|GetDataTableRow` "/Game/DirectionalCombat/Blueprints/Data/DataTables/DT_Weapons.DT_Weapons" _array_element)
      (:`then`
        (`KismetArrayLibrary.Array_AddUnique` (`self.Weapons`) _returnvalue)))))