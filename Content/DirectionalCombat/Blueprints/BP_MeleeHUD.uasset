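; HUD for directional melee combat that shows the player's Top, Right or Left aim direction through a W_AimDirection widget.
; Aim raises the chosen indicator to full opacity, and EndAim dims all three.
; ActivateAim reads the player character's status message to tint the aimed indicator for attack or defence, and DeactivateAim restores the inactive tint.
; The weapon and status functions are empty or default-returning stubs.
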(event `self.ReceiveBeginPlay`
  ;[1 1 1] Create Aim Wiget
  (bind _returnvalue (`|CreateWidget` "/Game/DirectionalCombat/Art/W_AimDirection.W_AimDirection_C" (`GameplayStatics.GetPlayerController` 0)))
  (bind _output_get (set `self.AimDirectionWiget` _returnvalue))
  (`UserWidget.AddToViewport` _output_get 0)
  (`self.EndAim`))

(event `self.Aim`
  (params (AimDirection :type "/Game/DirectionalCombat/Blueprints/Data/E_AimDirection Enum" :default "NewEnumerator0"))
  (bind _aimdirectionwiget (`self.AimDirectionWiget`))
  ;[1 1 1] Update Wiget Opacity By Direction
  (`self.EndAim`)
  (`Image.SetOpacity` (select `/Game/DirectionalCombat/Blueprints/Data/E_AimDirection` AimDirection :`NewEnumerator0` (`/Game/DirectionalCombat/Art/W_AimDirection.Top` _aimdirectionwiget) :`NewEnumerator1` (`/Game/DirectionalCombat/Art/W_AimDirection.Right` _aimdirectionwiget) :`NewEnumerator2` (`/Game/DirectionalCombat/Art/W_AimDirection.Left` _aimdirectionwiget)) 1.0))

(event `self.EndAim`
  (bind _aimdirectionwiget (`self.AimDirectionWiget`))
  ;[1 1 1] Reset Wigets
  (for _index (range 3)
    (`Image.SetOpacity` (select `int` _index :`0` (`/Game/DirectionalCombat/Art/W_AimDirection.Top` _aimdirectionwiget) :`1` (`/Game/DirectionalCombat/Art/W_AimDirection.Right` _aimdirectionwiget) :`2` (`/Game/DirectionalCombat/Art/W_AimDirection.Left` _aimdirectionwiget)) 0.5)))

(event `self.ActivateAim`
  (bind _aimdirectionwiget (`self.AimDirectionWiget`))
  ;[1 1 1] Alter Wiget Coler Based on Input
  (bind (_hasweapon _isattacking _isblocking _iskicking _isprepared _aimdirection) (message `/Game/DirectionalCombat/Blueprints/Interfaces/I_Combat.GetCharacterStatus` (`GameplayStatics.GetPlayerCharacter` 0)))
  (if _isattacking
    (bind _returnvalue (select `/Game/DirectionalCombat/Blueprints/Data/E_AimDirection` _aimdirection :`NewEnumerator0` (`/Game/DirectionalCombat/Art/W_AimDirection.Top` _aimdirectionwiget) :`NewEnumerator1` (`/Game/DirectionalCombat/Art/W_AimDirection.Right` _aimdirectionwiget) :`NewEnumerator2` (`/Game/DirectionalCombat/Art/W_AimDirection.Left` _aimdirectionwiget)))
    (`Image.SetBrushTintColor` _returnvalue (`self.AttackColor`))
    (else
      (`Image.SetBrushTintColor` _returnvalue (`self.Defence Color`)))))

(event `self.DeactivateAim`
  (bind _aimdirectionwiget (`self.AimDirectionWiget`))
  ;[1 1 1] Reset Wiget Color
  (for _index (range 3)
    (`Image.SetBrushTintColor` (select `int` _index :`0` (`/Game/DirectionalCombat/Art/W_AimDirection.Top` _aimdirectionwiget) :`1` (`/Game/DirectionalCombat/Art/W_AimDirection.Right` _aimdirectionwiget) :`2` (`/Game/DirectionalCombat/Art/W_AimDirection.Left` _aimdirectionwiget)) (`self.DeactiveColor`))))

(fn `Edit Weapon`
  (params (CurrWeapon :type "/Game/DirectionalCombat/Blueprints/Data/S_Weapon Structure") (EditType :type "/Game/DirectionalCombat/Blueprints/Data/E_Upgrades Enum" :default "NewEnumerator0"))
  (returns (UpgradedWeapon :type "/Game/DirectionalCombat/Blueprints/Data/S_Weapon Structure"))
  (return))

(fn `GetCharacterStatus`
  (returns (HasWeapon :type Boolean) (IsAttacking :type Boolean) (IsBlocking :type Boolean) (IsKicking :type Boolean) (isPrepared :type Boolean) (AimDirection :type "/Game/DirectionalCombat/Blueprints/Data/E_AimDirection Enum"))
  (return false false false false false "NewEnumerator0"))

(fn `GetWeapon`
  (returns (CurWeapon :type "/Game/DirectionalCombat/Blueprints/Data/S_Weapon Structure"))
  (return))

(fn `SetWeapon`
  (params (WeaponIndex :type Integer))
  (returns (NewCurrWeapon :type "/Game/DirectionalCombat/Blueprints/Data/S_Weapon Structure"))
  (return))

(fn `UserConstructionScript`)