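; Base combat entity Blueprint for directional combat, handling sprint toggle, attack, kick, block and weapon switching.
; Boolean state flags gate conflicting actions; attack and kick disable movement, and GetCharacterStatus reports the flags plus weapon possession.
; Weapon switching notifies the anim instance and Weapon component, while Edit, Get and SetWeapon are empty stubs.
; Data Table-driven body-part health and mesh setup, plus point-damage binding, exist but are disconnected.
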(event `self.ReceiveBeginPlay`
  (set `self.AnimInstance` (`SkeletalMeshComponent.GetAnimInstance` (`self.CoreMesh`)))
  (bind _asskeletal_mesh_component (cast `SkeletalMeshComponent` (`|GetArrayItem` (`self.GetComponentsByTag` "/Script/Engine.ActorComponent" "Torso"))))
  (`SkinnedMeshComponent.SetSkinnedAssetAndUpdate` _asskeletal_mesh_component null true)
  (for _array_element (`self.GetComponentsByTag` "/Script/Engine.ActorComponent" "Head")
    (cast `SkeletalMeshComponent` _array_element)))

(event `Take Damage` :!signature `self.OnTakePointDamage`
  (params (DamagedActor :type "Actor Object Reference") (Damage :type "Float (double-precision)") (InstigatedBy :type "Controller Object Reference") (HitLocation :type "Vector Structure") (FHitComponent :type "PrimitiveComponent Object Reference") (BoneName :type Name) (ShotFromDirection :type "Vector Structure") (DamageType :type "DamageType Object Reference") (DamageCauser :type "Actor Object Reference"))
  (bind _output_get (set `self.ComponentHit` FHitComponent))
  (`KismetSystemLibrary.PrintString` (`KismetSystemLibrary.GetDisplayName` _output_get)))

(event `Sprint`
  (bind _charactermovement (`self.CharacterMovement`))
  ;[1 1 1] Sprint
  (`/Engine/EditorBlueprintResources/StandardMacros.FlipFlop`
    (:`A`
      (set `CharacterMovementComponent.MaxWalkSpeed` (`self.Sprint Speed`) _charactermovement))
    (:`B`
      (set `CharacterMovementComponent.MaxWalkSpeed` (`self.Walk Speed`) _charactermovement))))

(event `Attack`
  ;[1 1 1] Attack
  (if (not (or (`self.isSwitching`) (or (`self.IsKicking`) (or (`self.IsAttacking`) (`self.IsBlocking`)))))
    (set `self.IsAttacking` true)
    (`CharacterMovementComponent.DisableMovement` (`self.CharacterMovement`))))

(event `StartKick`
  ;[1 1 1] Kick
  (set `self.IsKicking` true)
  (`CharacterMovementComponent.DisableMovement` (`self.CharacterMovement`)))

(event `/Game/DirectionalCombat/Blueprints/Interfaces/I_Combat.Kick`
  ;[1 1 1] Kick
  (set `self.IsKicking` false))

(event `/Game/DirectionalCombat/Blueprints/Interfaces/I_Combat.DeactivateAim`
  ;[1 1 1] Attack
  (set `self.IsAttacking` false))

(event `Block`
  (params (IsPressed :type Boolean))
  (bind _returnvalue (or (or (`self.IsAttacking`) (`self.IsKicking`)) (`self.isSwitching`)))
  ;[1 1 1] Block
  (if IsPressed
    (if (not _returnvalue)
      (set `self.IsBlocking` true))
    (elif (not _returnvalue)
      (set `self.IsBlocking` false))))

(event `Switch Weapon`
  ;[1 1 1] Switch Weapon
  (if (not (or (`self.isSwitching`) (or (`self.IsKicking`) (or (`self.IsAttacking`) (`self.IsBlocking`)))))
    (set `self.isSwitching` true)
    (message `/Game/DirectionalCombat/Blueprints/Interfaces/I_Combat.SwitchWeapon` (`SkeletalMeshComponent.GetAnimInstance` (`self.CoreMesh`)))
    (`/Game/DirectionalCombat/Blueprints/BP_WepHolder.Switch Weapon` (`self.Weapon`))))

(fn `Edit Weapon`
  (params (CurrWeapon :type "/Game/DirectionalCombat/Blueprints/Data/S_Weapon Structure") (EditType :type "/Game/DirectionalCombat/Blueprints/Data/E_Upgrades Enum" :default "NewEnumerator0"))
  (returns (UpgradedWeapon :type "/Game/DirectionalCombat/Blueprints/Data/S_Weapon Structure"))
  (return))

(fn `GetCharacterStatus`
  (returns (HasWeapon :type Boolean) (IsAttacking :type Boolean) (IsBlocking :type Boolean) (IsKicking :type Boolean) (isPrepared :type Boolean) (AimDirection :type "/Game/DirectionalCombat/Blueprints/Data/E_AimDirection Enum"))
  (if (!= (`.Index_31_9DE60E67468BFA8216A140B084BAFE3B` (break `/Game/DirectionalCombat/Blueprints/Data/S_Weapon` (`/Game/DirectionalCombat/Blueprints/BP_WepHolder.CurrWeapon` (`self.Weapon`)))) 0)
    (set `self.HasWeapon` true)
    (else
      (bind _output_get (set `self.HasWeapon` false))))
  (return _output_get (`self.IsAttacking`) (`self.IsBlocking`) (`self.IsKicking`) true "NewEnumerator0"))

(fn `GetWeapon`
  (returns (CurWeapon :type "/Game/DirectionalCombat/Blueprints/Data/S_Weapon Structure"))
  (return))

(fn `SetWeapon`
  (params (WeaponIndex :type Integer))
  (returns (NewCurrWeapon :type "/Game/DirectionalCombat/Blueprints/Data/S_Weapon Structure"))
  (return))

(fn `UserConstructionScript`
  (locals (CurrentComponent :type "SkeletalMeshComponent Object Reference") (CurrentBodyPart :type "/Game/DirectionalCombat/Blueprints/Data/S_BodyPart Structure")))