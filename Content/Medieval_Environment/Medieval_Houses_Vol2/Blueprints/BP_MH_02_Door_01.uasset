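; BP_MH_02_Door_01 is a medieval house wooden door that swings open when an actor enters its detection sphere and closes when one leaves.
; A timeline drives DoorLeft's yaw up to 92 degrees, playing on overlap and reversing on exit.
; The IsActorOnPosY result picks the swing direction from the overlapping actor.
; The construction script sets the sphere radius and selects one of three door meshes by clamped DoorType.
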(event `self.Sphere.OnComponentBeginOverlap`
  (params (OverlappedComponent :type "PrimitiveComponent Object Reference") (OtherActor :type "Actor Object Reference") (OtherComp :type "PrimitiveComponent Object Reference") (OtherBodyIndex :type Integer) (bFromSweep :type Boolean) (SweepResult :type "HitResult Structure (by ref)"))
  (set `self.NegY` (`self.IsActorOnPosY` OtherActor))
  (bind (_direction _rotationcoeff) (`Timeline|Timeline_Rotation` :!label _label)
    (:`Update`
      (bind _returnvalue (* _rotationcoeff 92.0))
      (`SceneComponent.K2_SetRelativeRotation` (`self.Door_Left`) (`KismetMathLibrary.MakeRotator` 0.0 0.0 (`KismetMathLibrary.SelectFloat` _returnvalue (* _returnvalue -1.0) (`self.NegY`))) false false))))

(event `self.Sphere.OnComponentEndOverlap`
  (params (OverlappedComponent :type "PrimitiveComponent Object Reference") (OtherActor :type "Actor Object Reference") (OtherComp :type "PrimitiveComponent Object Reference") (OtherBodyIndex :type Integer))
  (goto _label :!via `Reverse`))

(fn `UserConstructionScript`
  (`SphereComponent.SetSphereRadius` (`self.Sphere`) (`self.DetectionRadius`) true)
  (bind _output_get (set `self.DoorType` (`KismetMathLibrary.Clamp` (`self.DoorType`) 0 2)))
  (switch `int` _output_get
    (:`0`
      (`StaticMeshComponent.SetStaticMesh` (`self.Door_Left`) "/Game/Medieval_Environment/Medieval_Houses_Vol2/Meshes/SM_MH_02_Wood_Door_01.SM_MH_02_Wood_Door_01"))
    (:`1`
      (`StaticMeshComponent.SetStaticMesh` (`self.Door_Left`) "/Game/Medieval_Environment/Medieval_Houses_Vol2/Meshes/SM_MH_02_Wood_Door_02.SM_MH_02_Wood_Door_02"))
    (:`2`
      (`StaticMeshComponent.SetStaticMesh` (`self.Door_Left`) "/Game/Medieval_Environment/Medieval_Houses_Vol2/Meshes/SM_MH_02_Wood_Door_03.SM_MH_02_Wood_Door_03"))))