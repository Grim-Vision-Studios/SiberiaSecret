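; BP_WepHolder is a weapon holder that keeps a slot-indexed array of stored weapons and tracks the equipped one.
; SwitchWeapon hides the current weapon actor and makes the entry at the equipped index current, without changing the index or unhiding the new weapon.
; AssignWeapon writes a weapon into a given slot after a bounds check, printing an error when the index is invalid.
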(fn `AssignWeapon`
  (params (AssignSlot :type Integer) (NewWeaponStats :type "/Game/InStudio/Blueprints/SevereCombat/Weapons/BP_Weapon_Base Object Reference"))
  (if (`KismetArrayLibrary.Array_IsValidIndex` (`self.StoredWeapons`) AssignSlot)
    (`KismetArrayLibrary.Array_Set` (`self.StoredWeapons`) AssignSlot NewWeaponStats)
    (else
      (`KismetSystemLibrary.PrintString` "Error: Out of bounds index." true true (struct :`R` 1.0 :`B` 0.641949 :`A` 1.0)))))

(fn `SwitchWeapon`
  (`Actor.SetActorHiddenInGame` (`self.EquipedWeapon`) true)
  (set `self.EquipedWeapon` (`|GetArrayItem` (`self.StoredWeapons`) (`self.EquipedIndex`))))