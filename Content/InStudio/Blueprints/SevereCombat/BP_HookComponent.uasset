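; Grappling hook component that either pulls its owner to Hookable surfaces or drags Pullable static mesh actors to itself.
; Hook sphere-traces along the camera's forward vector and branches on the hit's object type, range-checking Hookable hits in 2D.
; Tick repeats frame-time lerps until arrival within a radius.
; Owner collision is disabled while grappling to above the impact point, and pulled meshes' physics is suspended until arrival.
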(event `self.ReceiveBeginPlay`
  (`KismetSystemLibrary.PrintString` "Hook comp"))

(event `Hook`
  (params (CameraComp :type "CameraComponent Object Reference"))
  (bind (_outhit _hashit) (`self.Trace Grapple` CameraComp))
  (if _hashit
    (set `self.HasHit` _hashit)
    (bind (_bblockinghit _binitialoverlap _time _distance _location _impactpoint _normal _impactnormal _physmat _hitactor _hitcomponent) (`GameplayStatics.BreakHitResult` _outhit))
    (switch `ECollisionChannel` (`PrimitiveComponent.GetCollisionObjectType` _hitcomponent)
      (:`ECC_GameTraceChannel1`
        (if (`self.DistanceCheck` _impactpoint (`self.hookDistanceRange`))
          (bind _location_2 (`self.Grapple` _impactpoint (stale `self.ReceiveTick` DeltaSeconds) :!label _label))
          (`Actor.K2_SetActorLocation` (`self.GetOwner`) _location_2 false false)
          (else
            (set `self.HasHit` false))))
      (:`ECC_GameTraceChannel2`
        (bind _location_3 (`self.Pull` _hitactor (stale `self.ReceiveTick` DeltaSeconds) :!label _label_2))
        (`Actor.K2_SetActorLocation` _hitactor _location_3 false true)))
    (else
      (set `self.HasHit` false))))

(event `self.ReceiveTick`
  (params (DeltaSeconds :type "Float (single-precision)"))
  (if (`self.HasHit`)
    (bind (_bblockinghit _binitialoverlap _time _distance _location _impactpoint _normal _impactnormal _physmat _hitactor _hitcomponent) (`GameplayStatics.BreakHitResult` (stale `Hook` _outhit)))
    (switch `ECollisionChannel` (`PrimitiveComponent.GetCollisionObjectType` _hitcomponent)
      (:`ECC_GameTraceChannel1`
        (if (`self.DestinationGrappleCheck` (`self.destination`) (`Actor.K2_GetActorLocation` (`self.GetOwner`)) 100.0)
          (`Actor.SetActorEnableCollision` (`self.GetOwner`) true)
          (set `self.HasHit` false)
          (else
            (goto _label))))
      (:`ECC_GameTraceChannel2`
        (if (`self.DestinationCheck` (`self.destination`) (`Actor.K2_GetActorLocation` _hitactor) 15.0)
          (bind _asstatic_mesh_actor (cast `StaticMeshActor` _hitactor))
          (`PrimitiveComponent.SetSimulatePhysics` (`StaticMeshActor.StaticMeshComponent` _asstatic_mesh_actor) true)
          (set `self.HasHit` false)
          (else
            (goto _label_2)))))))

(fn `DestinationCheck`
  (params (Destination :type "Vector Structure") (`Current Location` :type "Vector Structure") (Radius :type "Float (double-precision)"))
  (returns (IsCloseBy :type Boolean))
  (return (<= (`KismetMathLibrary.Vector_Distance` Destination `Current Location`) Radius)))

(fn `DestinationGrappleCheck`
  (params (Destination :type "Vector Structure") (CurrentLocation :type "Vector Structure") (Radius :type "Float (double-precision)"))
  (returns (IsCloseBy :type Boolean))
  (return (<= (`KismetMathLibrary.Vector_Distance` Destination CurrentLocation) Radius)))

(fn `DistanceCheck`
  (params (Location :type "Vector Structure") (Range :type "Float (double-precision)"))
  (returns (IsCloseBy :type Boolean))
  (return (<= (`KismetMathLibrary.Vector_Distance2D` Location (`Actor.K2_GetActorLocation` (`self.GetOwner`))) Range)))

(fn `Grapple`
  (params (ToLocation :type "Vector Structure") (DeltaTime :type "Float (double-precision)"))
  (returns (Location :type "Vector Structure"))
  (bind _returnvalue (`self.GetOwner`))
  (bind _returnvalue_2 (`KismetMathLibrary.MakeVector` (.x ToLocation) (.y ToLocation) (+ (.z ToLocation) 200.0)))
  (`Actor.SetActorEnableCollision` _returnvalue false)
  (set `self.destination` _returnvalue_2)
  (return (`KismetMathLibrary.VLerp` (`Actor.K2_GetActorLocation` _returnvalue) _returnvalue_2 (* DeltaTime (`self.HookTravelSpeed`)))))

(fn `Pull`
  (params (Actor :type "Actor Object Reference") (DeltaTime :type "Float (double-precision)"))
  (returns (Location :type "Vector Structure"))
  (bind _returnvalue (`self.K2_GetComponentLocation`))
  (bind _returnvalue_2 (`Actor.K2_GetActorLocation` Actor))
  (bind _returnvalue_3 (`KismetMathLibrary.MakeVector` (.x (`self.K2_GetComponentLocation`)) (.y (`self.K2_GetComponentLocation`)) (+ (.z _returnvalue_2) 5.0)))
  (bind _asstatic_mesh_actor (cast `StaticMeshActor` Actor))
  (`PrimitiveComponent.SetSimulatePhysics` (`StaticMeshActor.StaticMeshComponent` _asstatic_mesh_actor) false)
  (if (`self.useActorZ`)
    (set `self.destination` _returnvalue_3)
    (return (`KismetMathLibrary.VLerp` _returnvalue_2 _returnvalue_3 (* DeltaTime (`self.PullTravelSpeed`))))
    (else
      (set `self.destination` _returnvalue)
      (return (`KismetMathLibrary.VLerp` (`Actor.K2_GetActorLocation` Actor) _returnvalue (* DeltaTime (`self.PullTravelSpeed`)))))))

(fn `Trace Grapple`
  (params (CameraComp :type "CameraComponent Object Reference"))
  (returns (OutHit :type "HitResult Structure") (HasHit :type Boolean))
  (bind _returnvalue (`self.K2_GetComponentLocation` CameraComp))
  (bind (_outhit _returnvalue_2) (`KismetSystemLibrary.SphereTraceSingleForObjects` _returnvalue (+ _returnvalue (* (`self.GetForwardVector` CameraComp) (`self.maxHookDistance`))) (`self.hookRadius`) (`self.Object Types`) true))
  (return _outhit _returnvalue_2))