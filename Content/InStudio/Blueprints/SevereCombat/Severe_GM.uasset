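; Game mode for the SevereCombat content that persists the player's respawn point through a BP_SiberiaSaveGame slot.
; On BeginPlay it loads the current slot, or creates one seeded with the PlayerStart transform without applying it to the player.
; LoadGame and SaveGame copy the respawn transform between the save and BP_Entity_Player.
; DeleteSave clears a hardcoded "Save1" slot rather than using CurrSaveName.
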(event `self.ReceiveBeginPlay`
  (bind _returnvalue (`GameplayStatics.DoesSaveGameExist` (`self.CurrSaveName`)))
  (if _returnvalue
    (`self.LoadGame`)
    (else
      (bind _returnvalue_2 (`GameplayStatics.GetActorOfClass` "/Script/Engine.PlayerStart"))
      (bind _returnvalue_3 (`GameplayStatics.CreateSaveGameObject` "/Game/InStudio/Blueprints/BP_SiberiaSaveGame.BP_SiberiaSaveGame_C"))
      (set `/Game/InStudio/Blueprints/BP_SiberiaSaveGame.RespawnTransform` (`self.GetTransform` _returnvalue_2) _returnvalue_3)
      (`GameplayStatics.SaveGameToSlot` _returnvalue_3 (`self.CurrSaveName`)))))

(event `LoadGame`
  (bind _returnvalue (`GameplayStatics.LoadGameFromSlot` (`self.CurrSaveName`)))
  (bind _asbp_siberia_save_game (cast `/Game/InStudio/Blueprints/BP_SiberiaSaveGame` _returnvalue))
  (bind _asbp_entity_player (cast `/Game/InStudio/Blueprints/SevereCombat/Entities/BP_Entity_Player` (`GameplayStatics.GetPlayerCharacter` 0)))
  (set `/Game/InStudio/Blueprints/SevereCombat/Entities/BP_Entity_Player.RespawnPoint` (`/Game/InStudio/Blueprints/BP_SiberiaSaveGame.RespawnTransform` _asbp_siberia_save_game) _asbp_entity_player))

(event `SaveGame`
  (bind _asbp_entity_player (cast `/Game/InStudio/Blueprints/SevereCombat/Entities/BP_Entity_Player` (`GameplayStatics.GetPlayerCharacter` 0)))
  (bind _returnvalue (`GameplayStatics.LoadGameFromSlot` (`self.CurrSaveName`)))
  (bind _asbp_siberia_save_game (cast `/Game/InStudio/Blueprints/BP_SiberiaSaveGame` _returnvalue))
  (set `/Game/InStudio/Blueprints/BP_SiberiaSaveGame.RespawnTransform` (`/Game/InStudio/Blueprints/SevereCombat/Entities/BP_Entity_Player.RespawnPoint` _asbp_entity_player) _asbp_siberia_save_game)
  (`GameplayStatics.SaveGameToSlot` _returnvalue (`self.CurrSaveName`)))

(event `DeleteSave`
  (`GameplayStatics.DeleteGameInSlot` "Save1"))

(fn `UserConstructionScript`)