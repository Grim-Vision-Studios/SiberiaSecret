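; Skeletal mesh component for one body part in the severe combat system, with its own health and dismemberment.
; It stores part type, health and an armor flag, exchanged through data setters and getters, with health starting at max.
; TakeDamage clamps health, optionally prints it for debugging, and returns true at zero.
; SevereLimb clears the leader pose, detaches the mesh and enables physics simulation so the limb separates.
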(event `self.ReceiveBeginPlay`
  (set `self.Health` (`self.MaxHealth`)))

(fn `GetPartData`
  (returns (PartData :type "/Game/InStudio/Blueprints/SevereCombat/Data/S_BodyPartData Structure"))
  (return (make `/Game/InStudio/Blueprints/SevereCombat/Data/S_BodyPartData` (`self.BodyPartType`) (`self.Health`) (`self.bHasArmor`))))

(fn `SetPartData`
  (params (S_BodyPart :type "/Game/InStudio/Blueprints/SevereCombat/Data/S_BodyPartData Structure (by ref)"))
  (bind (_bodyparttype _health _hasarmor) (break `/Game/InStudio/Blueprints/SevereCombat/Data/S_BodyPartData` S_BodyPart))
  (set `self.BodyPartType` _bodyparttype)
  (set `self.Health` _health)
  (set `self.bHasArmor` _hasarmor))

(fn `SevereLimb`
  (`self.SetLeaderPoseComponent` null)
  (`self.K2_DetachFromComponent` self "KeepRelative" "KeepRelative" "KeepRelative" true)
  (`self.SetSimulatePhysics` true))

(fn `TakeDamage`
  (params (DamageDelt :type "Float (double-precision)"))
  (returns (IsDead :type Boolean))
  (bind _output_get (set `self.Health` (`KismetMathLibrary.FClamp` (- (`self.Health`) DamageDelt) 0.0 (`self.MaxHealth`))))
  (if (`self.bDebug`)
    (`KismetSystemLibrary.PrintString` (`KismetStringLibrary.Concat_StrStr` (`KismetSystemLibrary.GetDisplayName` (`self.GetOwner`)) ": Health is at " (`KismetStringLibrary.Conv_DoubleToString` _output_get))))
  (if (== (`self.Health`) 0.0)
    (return true)
    (else
      (return false))))