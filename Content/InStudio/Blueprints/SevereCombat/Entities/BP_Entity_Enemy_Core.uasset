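; Core enemy entity for SevereCombat that models its body as separate BPC_BodyPart components with their own health and armor.
; The construction script gathers parts tagged Torso, Head or Limb, initializes each from EntityTable rows matching its body part type, and registers it in BodyParts.
; DamageLimb forwards damage to the registered part that was hit.
; Its point-damage binding is disconnected and BeginPlay is empty, so this file never hooks it up.
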(event `self.ReceiveBeginPlay`)

(event `DamageLimb` :!signature `self.OnTakePointDamage`
  (params (DamagedActor :type "Actor Object Reference") (Damage :type "Float (single-precision)") (InstigatedBy :type "Controller Object Reference") (HitLocation :type "Vector Structure") (FHitComponent :type "PrimitiveComponent Object Reference") (BoneName :type Name) (ShotFromDirection :type "Vector Structure") (DamageType :type "DamageType Object Reference") (DamageCauser :type "Actor Object Reference"))
  (bind _bodyparts (`self.BodyParts`))
  (bind _asbpc_body_part (cast `/Game/InStudio/Blueprints/SevereCombat/BPC_BodyPart` FHitComponent))
  (if (`KismetArrayLibrary.Array_Contains` _bodyparts _asbpc_body_part)
    (`/Game/InStudio/Blueprints/SevereCombat/BPC_BodyPart.Take Damage` (`|GetArrayItem` _bodyparts (`KismetArrayLibrary.Array_Find` _bodyparts _asbpc_body_part)) Damage)))

(fn `InitializeBodyParts`
  (params (Torso :type "/Game/InStudio/Blueprints/SevereCombat/BPC_BodyPart Object Reference") (Heads :type "Array of /Game/InStudio/Blueprints/SevereCombat/BPC_BodyPart Object Reference") (Limbs :type "Array of /Game/InStudio/Blueprints/SevereCombat/BPC_BodyPart Object Reference"))
  (locals (CurrentComponent :type "/Game/InStudio/Blueprints/SevereCombat/BPC_BodyPart Object Reference") (RowNames :type "Array of Name") (CurrentBodyPartType :type "/Game/InStudio/Blueprints/SevereCombat/Data/E_BodyParts Enum"))
  (bind _currentcomponent (`local.CurrentComponent`))
  (bind _outrownames (`DataTableFunctionLibrary.GetDataTableRowNames` (`self.EntityTable`)))
  (set `local.RowNames` _outrownames)
  (`|ExecutionSequence`
    (:`then_0`
      (set `local.CurrentBodyPartType` "NewEnumerator2")
      (set `local.CurrentComponent` Torso)
      (for _array_element (`local.RowNames`) :!label _label
        (bind _returnvalue (`|GetDataTableRow` (`self.EntityTable`) _array_element)
          (:`then`
            (bind (_bodyparttype _health _armor) (break `/Game/InStudio/Blueprints/SevereCombat/Data/S_BodyPart` _returnvalue))
            (if (`|EnumEquality` (`local.CurrentBodyPartType`) _bodyparttype)
              (`/Game/InStudio/Blueprints/SevereCombat/BPC_BodyPart.Set Variables` _currentcomponent _bodyparttype _health _armor)
              (`KismetArrayLibrary.Array_AddUnique` (`self.BodyParts`) _currentcomponent))))))
    (:`then_1`
      (if (`KismetArrayLibrary.Array_IsNotEmpty` Heads)
        (set `local.CurrentBodyPartType` "NewEnumerator0")
        (for _array_element_2 Heads
          (set `local.CurrentComponent` _array_element_2)
          (goto _label)))
      (if (`KismetArrayLibrary.Array_IsNotEmpty` Limbs)
        (set `local.CurrentBodyPartType` "NewEnumerator1")
        (for _array_element_3 Limbs
          (set `local.CurrentComponent` _array_element_3)
          (goto _label))))))

(fn `UserConstructionScript`
  (bind _output (`|GetArrayItem` (`self.GetComponentsByTag` "/Game/InStudio/Blueprints/SevereCombat/BPC_BodyPart.BPC_BodyPart_C" "Torso")))
  (`/Engine/EditorBlueprintResources/StandardMacros.IsValid` _output
    (:`Is Valid`
      (`self.InitializeBodyParts` _output (`self.GetComponentsByTag` "/Game/InStudio/Blueprints/SevereCombat/BPC_BodyPart.BPC_BodyPart_C" "Head") (`self.GetComponentsByTag` "/Game/InStudio/Blueprints/SevereCombat/BPC_BodyPart.BPC_BodyPart_C" "Limb")))
    (:`Is Not Valid`
      (`KismetSystemLibrary.PrintString` "No Valid Torso SK"))))