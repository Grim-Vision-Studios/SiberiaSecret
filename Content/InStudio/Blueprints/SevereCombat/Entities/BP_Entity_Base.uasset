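; BP_Entity_Base is a base character for melee combat, holding action state for attacks, shove, block, stance, sprint and weapon handling.
; Events gate actions on a shared IsBusy flag and set state that GetCharacterStatus exposes, while EnterIdle resets it after attacks and blocks.
; The WeaponHolder component handles current and stored weapons for switch, drop and pickup.
; BeginPlay caches the torso's AM_FPMelee anim instance, whose after-swing timer each attack clears.
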(event `self.ReceiveBeginPlay`
  (bind _asam_fpmelee (cast `/Game/InStudio/Art/TempCharacter/Animations/AM_FPMelee` (`SkeletalMeshComponent.GetAnimInstance` (`self.BPC_BodyPart_Torso`))))
  (set `self.AnimInstance` _asam_fpmelee)
  (if (== (`.Index_31_9DE60E67468BFA8216A140B084BAFE3B` (break `/Game/InStudio/Blueprints/SevereCombat/Data/S_Weapon` (`/Game/InStudio/Blueprints/SevereCombat/BP_WepHolder.CurrWeapon` (`self.WeaponHolder`)))) 0)
    _))

(event `Sprint`
  (bind _charactermovement (`self.CharacterMovement`))
  ;[1 1 1] Sprint
  (`/Engine/EditorBlueprintResources/StandardMacros.FlipFlop`
    (:`A`
      (set `CharacterMovementComponent.MaxWalkSpeed` (`self.Sprint Speed`) _charactermovement))
    (:`B`
      (set `CharacterMovementComponent.MaxWalkSpeed` (`self.Walk Speed`) _charactermovement))))

(event `self.SetCanHit`
  (params (NewCanHit :type Boolean))
  ;[1 1 1] Set Attack States
  (set `self.CanHit` NewCanHit))

(event `self.SetCanAttack`
  (params (NewCanAttack :type Boolean))
  ;[1 1 1] Set Attack States
  (set `self.CanAttack` NewCanAttack))

(event `DoShove`
  ;[1 1 1] Shove
  (set `self.IsBusy` true))

(event `DoAttack`
  ;[1 1 1] Attack
  (if (and (not (`self.IsBusy`)) (`self.CanAttack`) (`self.IsPrepared`))
    (set `self.ActionType` (`self.SwingType`))
    (set `self.IsBusy` true)
    (set `self.CanAttack` false)
    (`KismetSystemLibrary.K2_ClearAndInvalidateTimerHandle` (`/Game/InStudio/Art/TempCharacter/Animations/AM_FPMelee.AfterSwingTimer` (`self.AnimInstance`)))))

(event `self.EndShove`
  ;[1 1 1] Shove
)

(event `self.EndAttack`
  ;[1 1 1] Attack
  (`self.EnterIdle`))

(event `SetStance`
  (params (NewPrepared :type Boolean))
  ;[1 1 1] ToggleStance
  (set `self.IsPrepared` NewPrepared))

(event `DoBlock`
  (params (IsPressed :type Boolean))
  ;[1 1 1] Block
  (if (`self.IsBusy`)
    _
    (elif IsPressed
      (bind _output_get (set `self.IsBlocking` true))
      (set `self.IsBusy` _output_get)
      (else
        (set `self.IsBlocking` false)
        (`self.EnterIdle`)))))

(event `TrySwitchWeapon`
  ;[1 1 1] Switch Weapon
  (if (and (not (== (`.Index_31_9DE60E67468BFA8216A140B084BAFE3B` (break `/Game/InStudio/Blueprints/SevereCombat/Data/S_Weapon` (`/Game/InStudio/Blueprints/SevereCombat/BP_WepHolder.StoredWeapon` (`self.WeaponHolder`)))) 0)) (not (`self.IsBusy`)))
    (bind _output_get (set `self.isSwitching` true))
    (set `self.IsBusy` _output_get)))

(event `DropWeapon`
  ;[1 1 1] Drop Weapon
  (if (not (`self.IsBusy`))
    (`/Game/InStudio/Blueprints/SevereCombat/BP_WepHolder.Drop Curr Weapon` (`self.WeaponHolder`) (+ (`self.K2_GetActorLocation`) (* (`self.GetActorForwardVector`) 150.0)) (`self.K2_GetActorRotation`))
    (`self.UpdateWeapon`)))

(event `/Game/InStudio/Blueprints/SevereCombat/Interfaces/I_Intereactable.PickUpWeapon`
  (params (Weapon :type "/Game/InStudio/Blueprints/SevereCombat/Data/S_Weapon Structure"))
  ;[1 1 1] PickUpWeapon
  (if (not (== (`.Index_31_9DE60E67468BFA8216A140B084BAFE3B` (break `/Game/InStudio/Blueprints/SevereCombat/Data/S_Weapon` (`/Game/InStudio/Blueprints/SevereCombat/BP_WepHolder.CurrWeapon` (`self.WeaponHolder`)))) 0))
    (`self.DropWeapon`))
  (set `/Game/InStudio/Blueprints/SevereCombat/BP_WepHolder.CurrWeapon` Weapon (`self.WeaponHolder`))
  (`self.UpdateWeapon`))

(fn `EnterIdle`
  (set `self.ActionType` "NewEnumerator0")
  (set `self.IsBusy` false))

(fn `GetCharacterStatus`
  (returns (IsBlocking :type Boolean) (isPrepared :type Boolean) (IsSwitching :type Boolean) (AttackType :type "/Game/InStudio/Blueprints/SevereCombat/Data/E_ActionTypes Enum"))
  (return (`self.IsBlocking`) (`self.IsPrepared`) (`self.isSwitching`) (`self.ActionType`)))

(fn `GetWeapon`
  (returns (CurWeapon :type "/Game/InStudio/Blueprints/SevereCombat/Data/S_Weapon Structure"))
  (return))

(fn `Interact`
  (params (Owner :type "Actor Object Reference"))
  (returns (OtherActor :type "Actor Object Reference"))
  (return null))

(fn `SetWeapon`
  (params (WeaponIndex :type Integer))
  (returns (NewCurrWeapon :type "/Game/InStudio/Blueprints/SevereCombat/Data/S_Weapon Structure"))
  (return))

(fn `UserConstructionScript`
  (locals (CurrentComponent :type "SkeletalMeshComponent Object Reference") (CurrentBodyPart :type "/Game/InStudio/Blueprints/SevereCombat/Data/S_BodyPart Structure")))