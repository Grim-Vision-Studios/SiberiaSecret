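; BPC_BodyPart is a component that tracks health, armor and type for a single body part in the SevereCombat system.
; BeginPlay caches starting Health as MaxHealth, while SetVariables assigns type, Health and Armor without updating that maximum.
; TakeDamage subtracts raw damage, clamps Health between zero and MaxHealth and prints it.
; Armor is not applied to damage, and the zero-health branch is empty.
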(event `self.ReceiveBeginPlay`
  (set `self.MaxHealth` (`self.Health`)))

(event `Set Variables`
  (params (BodyPartType :type "/Game/InStudio/Blueprints/SevereCombat/Data/E_BodyParts Enum" :default "NewEnumerator1") (Health :type "Float (double-precision)") (Armor :type Integer))
  (set `self.BodyPartType` BodyPartType)
  (set `self.Health` Health)
  (set `self.Armor` Armor))

(event `Take Damage`
  (params (Damage :type "Float (double-precision)"))
  (bind _output_get (set `self.Health` (`KismetMathLibrary.FClamp` (- (`self.Health`) Damage) 0.0 (`self.MaxHealth`))))
  (`KismetSystemLibrary.PrintString` (`KismetStringLibrary.Conv_DoubleToString` _output_get))
  (if (== 0.0 (`self.Health`))
    _))