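; BP_WepHolder manages an owner's stored weapon data by slot and the weapon actor it currently holds.
; EquipWeapon, when nothing is held, async loads the slot's soft class, spawns a BP_Weapon_Base for the owner and applies its stored upgrades.
; Slot edits that hit the held slot trigger unequip or re-equip, but UnEquipWeapon is an empty stub and HeldSlot is never assigned here.
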(event `EquipWeapon`
  (params (Slot :type Integer))
  (bind _returnvalue (`self.GetOwner`))
  (bind (_output_name _output_description _output_icon _output_weaponclass _output_upgrades) (break `/Game/InStudio/Blueprints/SevereCombat/Data/S_WeaponData` (`|GetArrayItem` (`self.StoredWeapons`) Slot)))
  (`/Engine/EditorBlueprintResources/StandardMacros.IsValid` (`self.HeldWeapon`)
    (:`Is Not Valid`
      (if (`KismetSystemLibrary.IsValidSoftClassReference` _output_weaponclass)
        (bind _class (`|LoadAssetClass` _output_weaponclass)
          (:`Completed`
            (bind _asbp_weapon_base (castclass `/Game/InStudio/Blueprints/SevereCombat/Weapons/BP_Weapon_Base` _class))
            (bind _returnvalue_2 (`|SpawnActorFromClass` _asbp_weapon_base (`KismetMathLibrary.MakeTransform` (0.0 0.0 0.0)) "Undefined" "OverrideRootScale" _returnvalue (cast `Character` _returnvalue :!pure true)))
            (bind _output_get (set `self.HeldWeapon` _returnvalue_2))
            (`/Game/InStudio/Blueprints/SevereCombat/Weapons/BP_Weapon_Base.ApplyUpgrades` _output_get _output_upgrades)))))))

(fn `AddWeapon`
  (params (NewWeaponData :type "/Game/InStudio/Blueprints/SevereCombat/Data/S_WeaponData Structure"))
  (locals (NewData :type "/Game/InStudio/Blueprints/SevereCombat/Data/S_WeaponData Structure"))
  (bind _output_get (set `local.NewData` NewWeaponData))
  (`KismetArrayLibrary.Array_AddUnique` (`self.StoredWeapons`) _output_get))

(fn `ReEquipWeapon`
  (`self.UnEquipWeapon`)
  (`self.EquipWeapon` (`self.HeldSlot`)))

(fn `RemoveWeapon`
  (params (Slot :type Integer))
  (locals (NewSlot :type Integer))
  (bind _output_get (set `local.NewSlot` Slot))
  (`KismetArrayLibrary.Array_Set` (`self.StoredWeapons`) _output_get)
  (if (== _output_get (`self.HeldSlot`))
    (`self.UnEquipWeapon`)))

(fn `UnEquipWeapon`)

(fn `UpdateWeaponUpgrades`
  (params (Slot :type Integer) (Upgrades :type "/Game/InStudio/Blueprints/SevereCombat/Data/S_WeaponUpgrades Structure"))
  (setmembers `/Game/InStudio/Blueprints/SevereCombat/Data/S_WeaponData` :`StructRef` (`|GetArrayItem` (`self.StoredWeapons`) Slot) :`Upgrades` Upgrades)
  (if (== Slot (`self.HeldSlot`))
    (`self.ReEquipWeapon`)))