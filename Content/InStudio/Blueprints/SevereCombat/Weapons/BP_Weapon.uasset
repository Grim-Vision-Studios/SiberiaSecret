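; BP_Weapon is a weapon actor in the SevereCombat set, holding name, energy, stun level, damage, speed and mesh stats.
; ApplyDefaultStats loads the DT_Weapons row selected by StartWeaponIndex through SetStats and applies its skeletal mesh, while GetStats repacks the stats into a struct.
; Equip snaps to a body part's WeaponGrip socket.
; Drop detaches the owner actor and sweeps the weapon to a given transform; Interact is an empty stub.
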(event `Drop`
  (params (Location :type "Vector Structure") (Rotation :type "Rotator Structure"))
  (`self.K2_DetachFromActor` (`self.GetOwner`) "KeepRelative" "KeepRelative" "KeepRelative")
  (`self.K2_SetActorLocationAndRotation` Location Rotation true true))

(fn `ApplyDefaultStats`
  (bind _outrownames (`DataTableFunctionLibrary.GetDataTableRowNames` "/Game/InStudio/Blueprints/SevereCombat/Data/DataTables/DT_Weapons.DT_Weapons"))
  (bind _returnvalue (`|GetDataTableRow` "/Game/InStudio/Blueprints/SevereCombat/Data/DataTables/DT_Weapons.DT_Weapons" (`|GetArrayItem` _outrownames (`self.StartWeaponIndex`)))
    (:`then`
      (`self.SetStats` _returnvalue)
      (`SkinnedMeshComponent.SetSkinnedAssetAndUpdate` (`self.WeaponMesh`) (`self.Mesh`) true))))

(fn `Equip`
  (params (BodyPart :type "/Game/InStudio/Blueprints/SevereCombat/BPC_BodyPart Object Reference"))
  (`self.K2_AttachToComponent` BodyPart "WeaponGrip" "SnapToTarget" "SnapToTarget" "KeepWorld"))

(fn `GetStats`
  (returns (WeaponStats :type "/Game/InStudio/Blueprints/SevereCombat/Data/S_Weapon Structure"))
  (return (make `/Game/InStudio/Blueprints/SevereCombat/Data/S_Weapon` (`self.Name`) (`self.MaxEnergy`) (`self.Energy`) (`self.StunLevel`) (`self.Damage`) (`self.Speed`) (`self.Mesh`))))

(fn `Interact`
  (returns (IsWeapon :type Boolean)))

(fn `SetStats`
  (params (NewStats :type "/Game/InStudio/Blueprints/SevereCombat/Data/S_Weapon Structure"))
  (bind (_name _maxenergy _energy _stunlevel _damage _speed _mesh) (break `/Game/InStudio/Blueprints/SevereCombat/Data/S_Weapon` NewStats))
  (set `self.Name` _name)
  (set `self.MaxEnergy` _maxenergy)
  (set `self.Energy` _energy)
  (set `self.StunLevel` _stunlevel)
  (set `self.Damage` _damage)
  (set `self.Speed` _speed)
  (set `self.Mesh` _mesh))

(fn `UserConstructionScript`)