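; BP_Weapon_Base is a base weapon Blueprint for the SevereCombat code, holding a weapon's name, energy, stun level, damage and speed.
; SetStats and GetStats convert those variables from and to an SWeapon struct.
; Equip hides the actor and snaps a component to the WeaponGrip socket of the holding body part.
; Drop detaches the owner and sweeps the weapon to a given location and rotation, without unhiding it.
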(event `Drop`
  (params (Location :type "Vector Structure") (Rotation :type "Rotator Structure"))
  (`self.K2_DetachFromActor` (`self.GetOwner`) "KeepRelative" "KeepRelative" "KeepRelative")
  (`self.K2_SetActorLocationAndRotation` Location Rotation true true))

(event `Equip`
  (params (`Holding Body Part` :type "/Game/InStudio/Blueprints/SevereCombat/BPC_BodyPart Object Reference"))
  (`self.SetActorHiddenInGame` true)
  (`self.K2_AttachToComponent` `Holding Body Part` "WeaponGrip" "SnapToTarget" "SnapToTarget" "KeepWorld"))

(fn `GetStats`
  (returns (WeaponStats :type "/Game/InStudio/Blueprints/SevereCombat/Data/S_Weapon Structure"))
  (return (make `/Game/InStudio/Blueprints/SevereCombat/Data/S_Weapon` (`self.Name`) (`self.MaxEnergy`) (`self.Energy`) (`self.StunLevel`) (`self.Damage`) (`self.Speed`))))

(fn `SetStats`
  (params (NewStats :type "/Game/InStudio/Blueprints/SevereCombat/Data/S_Weapon Structure"))
  (bind (_name _maxenergy _energy _stunlevel _damage _speed) (break `/Game/InStudio/Blueprints/SevereCombat/Data/S_Weapon` NewStats))
  (set `self.Name` _name)
  (set `self.MaxEnergy` _maxenergy)
  (set `self.Energy` _energy)
  (set `self.StunLevel` _stunlevel)
  (set `self.Damage` _damage)
  (set `self.Speed` _speed))

(fn `UserConstructionScript`)