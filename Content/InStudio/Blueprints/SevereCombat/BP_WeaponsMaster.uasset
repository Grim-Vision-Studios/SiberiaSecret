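; Weapons master Blueprint that holds the combat weapon list and serves weapon data by index.
; The construction script reads every row of DT_Weapons and adds it uniquely to the Weapons array.
; SetWeapon and SetCurWeapon only return the array entry at the given index, despite their setter names.
; GetCharacterStatus returns fixed defaults and GetWeapon returns nothing, so both act as stubs.
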(fn `GetCharacterStatus`
  (returns (HasWeapon :type Boolean) (IsAttacking :type Boolean) (IsBlocking :type Boolean) (IsKicking :type Boolean) (isPrepared :type Boolean) (AimDirection :type "/Game/InStudio/Blueprints/SevereCombat/Data/E_AimDirection Enum"))
  (return false false false false false "NewEnumerator0"))

(fn `GetWeapon`
  (returns (CurWeapon :type "/Game/InStudio/Blueprints/SevereCombat/Data/S_Weapon Structure"))
  (return))

(fn `SetCurWeapon`
  (params (Index :type Integer))
  (returns (Output :type "/Game/InStudio/Blueprints/SevereCombat/Data/S_Weapon Structure"))
  (return (`|GetArrayItem` (`self.Weapons`) Index)))

(fn `SetWeapon`
  (params (WeaponIndex :type Integer))
  (returns (NewCurrWeapon :type "/Game/InStudio/Blueprints/SevereCombat/Data/S_Weapon Structure"))
  (return (`|GetArrayItem` (`self.Weapons`) WeaponIndex)))

(fn `UserConstructionScript`
  (bind _outrownames (`DataTableFunctionLibrary.GetDataTableRowNames` "/Game/InStudio/Blueprints/SevereCombat/Data/DataTables/DT_Weapons.DT_Weapons"))
  (for _array_element _outrownames
    (bind _returnvalue (`|GetDataTableRow` "/Game/InStudio/Blueprints/SevereCombat/Data/DataTables/DT_Weapons.DT_Weapons" _array_element)
      (:`then`
        (`KismetArrayLibrary.Array_AddUnique` (`self.Weapons`) _returnvalue)))))