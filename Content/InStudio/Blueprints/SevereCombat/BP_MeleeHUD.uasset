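; Melee combat HUD that creates the W_AimDirection widget on BeginPlay to display the player's aim axis.
; Aim events change the axis opacity, and SwitchAxis plays its animation forward for Idle or reversed for Horizontal.
; ShowAim queries the player character's status but branches on a constant true, so it always applies the attack tint, and EndAttack applies the inactive tint.
; The status and weapon functions are placeholder stubs.
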(event `self.ReceiveBeginPlay`
  ;[1 1 1] Create Aim Wiget
  (bind _returnvalue (`|CreateWidget` "/Game/InStudio/Art/UI/W_AimDirection.W_AimDirection_C" (`GameplayStatics.GetPlayerController` 0)))
  (bind _output_get (set `self.AimDirectionWiget` _returnvalue))
  (`UserWidget.AddToViewport` _output_get 0))

(event `self.Aim`
  (params (AimAxis :type "/Game/InStudio/Blueprints/SevereCombat/Data/E_AttackOrientation Enum" :default "NewEnumerator1"))
  ;[1 1 1] Set Wiget Opacity When ready
  (`Widget.SetRenderOpacity` (`/Game/InStudio/Art/UI/W_AimDirection.AimAxis` (`self.AimDirectionWiget`)) 0.9))

(event `SwitchAxis`
  (params (CurAimDirection :type "/Game/InStudio/Blueprints/SevereCombat/Data/E_AttackOrientation Enum" :default "NewEnumerator0"))
  (bind _aimdirectionwiget (`self.AimDirectionWiget`))
  (bind _changeaxis (`/Game/InStudio/Art/UI/W_AimDirection.ChangeAxis` _aimdirectionwiget))
  ;[1 1 1] Switch Wiget Axis
  (switch `/Game/InStudio/Blueprints/SevereCombat/Data/E_AttackOrientation` CurAimDirection
    (:`NewEnumerator1`
      (`UserWidget.PlayAnimationReverse` _aimdirectionwiget _changeaxis 1.0 false))
    (:`NewEnumerator0`
      (`UserWidget.PlayAnimationForward` _aimdirectionwiget _changeaxis 1.0 false))))

(event `self.EndAim`
  ;[1 1 1] Reset Wiget Opacity
  (`Image.SetOpacity` (`/Game/InStudio/Art/UI/W_AimDirection.AimAxis` (`self.AimDirectionWiget`)) 0.0))

(event `self.ShowAim`
  (bind _aimaxis (`/Game/InStudio/Art/UI/W_AimDirection.AimAxis` (`self.AimDirectionWiget`)))
  ;[1 1 1] Set New Wiget Color Based on Input
  (message `/Game/InStudio/Blueprints/SevereCombat/Interfaces/I_Combat.GetCharacterStatus` (`GameplayStatics.GetPlayerCharacter` 0))
  (if true
    (`Image.SetBrushTintColor` _aimaxis (`self.AttackColor`))
    (else
      (`Image.SetBrushTintColor` _aimaxis (`self.Defence Color`)))))

(event `self.EndAttack`
  ;[1 1 1] Reset Wiget Color
  (`Image.SetBrushTintColor` (`/Game/InStudio/Art/UI/W_AimDirection.AimAxis` (`self.AimDirectionWiget`)) (`self.DeactiveColor`)))

(fn `GetCharacterStatus`
  (returns (isPrepared :type Boolean) (AttackOrientation :type "/Game/InStudio/Blueprints/SevereCombat/Data/E_AttackOrientation Enum") (AttackType :type "/Game/InStudio/Blueprints/SevereCombat/Data/CombatActions/Actions_Base Object Reference") (AttackType :type "/Game/InStudio/Blueprints/SevereCombat/Data/E_AttackOrientation Enum"))
  (return false "NewEnumerator1" null "(INVALID)"))

(fn `GetWeapon`
  (returns (CurWeapon :type "/Game/InStudio/Blueprints/SevereCombat/Data/S_Weapon Structure"))
  (return))

(fn `SetWeapon`
  (params (WeaponIndex :type Integer))
  (returns (NewCurrWeapon :type "/Game/InStudio/Blueprints/SevereCombat/Data/S_Weapon Structure"))
  (return))

(fn `UserConstructionScript`)