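; AC_InteractWidget is a widget component that shows and hides an interact message.
; On BeginPlay it casts its widget to W_InteractMessage and caches the reference.
; ShowInteractMessage and HideInteractMessage play that widget's ShowInteract animation forward or in reverse, with an IsShown flag preventing repeat plays.
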(event `self.ReceiveBeginPlay`
  (bind _asw_interact_message (cast `/Game/InStudio/Art/UI/W_InteractMessage` (`self.GetWidget`)))
  (set `self.InteractMessageWidget` _asw_interact_message))

(event `ShowInteractMessage`
  (bind _interactmessagewidget (`self.InteractMessageWidget`))
  (if (not (`self.IsShown`))
    (set `self.IsShown` true)
    (`UserWidget.PlayAnimationForward` _interactmessagewidget (`/Game/InStudio/Art/UI/W_InteractMessage.ShowInteract` _interactmessagewidget) 1.0 false)))

(event `HideInteractMessage`
  (bind _interactmessagewidget (`self.InteractMessageWidget`))
  (if (`self.IsShown`)
    (set `self.IsShown` false)
    (`UserWidget.PlayAnimationReverse` _interactmessagewidget (`/Game/InStudio/Art/UI/W_InteractMessage.ShowInteract` _interactmessagewidget) 1.0 false)))