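; AC_Inventory is an inventory component that stores item objects in a slot array sized from columns times rows at BeginPlay.
; AddItem finds the first invalid slot, fills it through SetSlotItem and returns whether space was found.
; SetSlotItem fires the OnItemUpdated dispatcher with item and index, while RemoveItem clears a slot without notifying.
; DropItem is an empty stub.
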(event `self.ReceiveBeginPlay`
  (`KismetArrayLibrary.Array_Resize` (`self.ItemSlots`) (* (`self.Collums`) (`self.Rows`))))

(fn `AddItem`
  (params (ItemObject :type "/Game/InStudio/Blueprints/Items/BP_ItemObject Object Reference"))
  (returns (Success :type Boolean))
  (bind (_foundspace _foundindex) (`self.FindFirstOpenSlot`))
  (if _foundspace
    (`self.SetSlotItem` _foundindex ItemObject)
    (return true)
    (else
      (return false))))

(fn `DropItem`)

(fn `FindFirstOpenSlot`
  (returns (FoundSpace :type Boolean) (FoundIndex :type Integer))
  (for (_array_element _array_index) (`self.ItemSlots`)
    (`/Engine/EditorBlueprintResources/StandardMacros.IsValid` _array_element
      (:`Is Not Valid`
        (return true _array_index))))
  (return false 0))

(fn `RemoveItem`
  (params (StoredIndex :type Integer))
  (`KismetArrayLibrary.Array_Set` (`self.ItemSlots`) StoredIndex))

(fn `SetSlotItem`
  (params (StoredIndex :type Integer) (NewItemObject :type "/Game/InStudio/Blueprints/Items/BP_ItemObject Object Reference"))
  (`KismetArrayLibrary.Array_Set` (`self.ItemSlots`) StoredIndex NewItemObject)
  (`self.OnItemUpdated` NewItemObject StoredIndex))