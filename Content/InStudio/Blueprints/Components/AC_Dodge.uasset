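; Actor component that gives its owner a dodge on the IA_Dodge input, blocked while the owner's state is Actions.Attack.End.
; An impulse through the CharacterMovementComponent pushes along the last input vector, or backward when there is none, scaled by DodgePower.
; The owner's state switches to Dodge, returns to Idle after DodgeTime, and a DoOnce gate reopens after DodgeCooldown.
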(event `self.ReceiveBeginPlay`
  (set `self.MovementComponent` (`Actor.GetComponentByClass` (`self.GetOwner`) "/Script/Engine.CharacterMovementComponent")))

(event `EnhancedInput|/Game/InStudio/Input/Gameplay/IA_Dodge`
  (params (ActionValue :type Boolean) (ElapsedSeconds :type "Float (double-precision)") (TriggeredSeconds :type "Float (double-precision)") (InputAction :type "InputAction Object Reference" :default "/Game/InStudio/Input/Gameplay/IA_Dodge.IA_Dodge"))
  (bind _movementcomponent (`self.MovementComponent`))
  (bind _returnvalue (`PawnMovementComponent.GetLastInputVector` _movementcomponent))
  (:`Triggered`
    (bind _currentstate (message `/Game/InStudio/Blueprints/Interfaces/I_StateMachine.Get Current State` (`self.GetOwner`)))
    (if (not (`BlueprintGameplayTagLibrary.MatchesAnyTags` _currentstate (`BlueprintGameplayTagLibrary.MakeLiteralGameplayTagContainer` (struct :`GameplayTags` (struct :`(TagName` "Actions.Attack.End") :`(TagName` "Actions.Attack.Start")))) true))
      (`/Engine/EditorBlueprintResources/StandardMacros.DoOnce` false :!label _label
        (:`Completed`
          (message `/Game/InStudio/Blueprints/Interfaces/I_StateMachine.SwitchState` (`self.GetOwner`) (struct :`TagName` "Actions.Dodge"))
          (`CharacterMovementComponent.AddImpulse` _movementcomponent (* (* (select `bool` (== _returnvalue (0.0 0.0 0.0) :`ErrorTolerance` 0.01) :`false` _returnvalue :`true` (* (`Actor.GetActorForwardVector` (`self.GetOwner`)) -1)) 100000) (`self.DodgePower`)) false)
          (`KismetSystemLibrary.Delay` (`self.DodgeTime`))
          (message `/Game/InStudio/Blueprints/Interfaces/I_StateMachine.SwitchState` (`self.GetOwner`) (struct :`TagName` "Actions.Idle"))
          (`KismetSystemLibrary.Delay` (`self.DodgeCooldown`))
          (goto _label :!via `Reset`))))))