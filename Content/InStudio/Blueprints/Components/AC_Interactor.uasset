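; AC_Interactor is an actor component that lets its owner interact with overlapped actors that have an AC_Interactable component.
; Owner overlap events track a single current interactable, and the IA_Interact input calls Interact on it with the controller cached at BeginPlay.
; For player-controlled pawns only, it toggles the interactable's prompt and binds to OnUsedSet so the prompt follows the used state.
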(event `self.ReceiveBeginPlay`
  ;[1 1 1] Check If Controlled By Player
  (bind _aspawn (cast `Pawn` (`self.GetOwner`))
    (:`then`
      (set `self.IsPlayerControlled` (`Pawn.IsPlayerControlled` _aspawn))
      (set `self.OwnerController` (`Pawn.GetController` _aspawn)))
    (:`CastFailed`
      _))
  ;[1 1 1] Show Interactable
  (add `Actor.OnActorBeginOverlap` (`self.GetOwner`) (delegate `CheckOverlapForInteractable`))
  ;[1 1 1] Forget Interactable
  (add `Actor.OnActorEndOverlap` (`self.GetOwner`) (delegate `ForgetInteractabe`)))

(event `ForgetInteractabe`
  (params (OverlappedActor :type "Actor Object Reference") (OtherActor :type "Actor Object Reference"))
  (bind _currentinteractable (`self.CurrentInteractable`))
  ;[1 1 1] Forget Interactable
  (if (== OtherActor (`self.CurrentInteractable`))
    (if (`self.IsPlayerControlled`)
      (`/Game/InStudio/Blueprints/Components/AC_Interactable.SetShowInteract` _currentinteractable false)
      (remove `/Game/InStudio/Blueprints/Components/AC_Interactable.OnUsedSet` _currentinteractable (delegate `OnUsedSet_Event`)))
    (set `self.CurrentInteractable` null)))

(event `CheckOverlapForInteractable`
  (params (OverlappedActor :type "Actor Object Reference") (OtherActor :type "Actor Object Reference"))
  (bind _returnvalue (`Actor.GetComponentByClass` OtherActor "/Game/InStudio/Blueprints/Components/AC_Interactable.AC_Interactable_C"))
  (bind _currentinteractable (`self.CurrentInteractable`))
  ;[1 1 1] Show Interactable
  (`/Engine/EditorBlueprintResources/StandardMacros.IsValid` _returnvalue
    (:`Is Valid`
      (`/Engine/EditorBlueprintResources/StandardMacros.IsValid` _currentinteractable
        (:`Is Valid`
          (if (and (`self.IsPlayerControlled`) (not (`/Game/InStudio/Blueprints/Components/AC_Interactable.GetIsUsed` _currentinteractable)))
            (`/Game/InStudio/Blueprints/Components/AC_Interactable.SetShowInteract` (`self.CurrentInteractable`) true)))
        (:`Is Not Valid`
          (`self.SetCurrentInteractable` _returnvalue))))))

(event `SetCurrentInteractable`
  (params (CurrentInteractable :type "/Game/InStudio/Blueprints/Components/AC_Interactable Object Reference"))
  ;[1 1 1] Set Interactable
  (set `self.CurrentInteractable` CurrentInteractable)
  ;[1 1 1] Listen For On Used
  (if (`self.IsPlayerControlled`)
    (add `/Game/InStudio/Blueprints/Components/AC_Interactable.OnUsedSet` (`self.CurrentInteractable`) (delegate `OnUsedSet_Event`))))

(event `OnUsedSet_Event`
  (params (IsUsed :type Boolean))
  ;[1 1 1] Listen For On Used
  (`/Game/InStudio/Blueprints/Components/AC_Interactable.SetShowInteract` (`self.CurrentInteractable`) (not IsUsed)))

(event `EnhancedInput|/Game/InStudio/Input/Actions/IA_Interact`
  (params (ActionValue :type Boolean) (ElapsedSeconds :type "Float (double-precision)") (TriggeredSeconds :type "Float (double-precision)") (InputAction :type "InputAction Object Reference" :default "/Game/InStudio/Input/Actions/IA_Interact.IA_Interact"))
  (bind _currentinteractable (`self.CurrentInteractable`))
  (:`Triggered`
    (`/Engine/EditorBlueprintResources/StandardMacros.IsValid` _currentinteractable
      (:`Is Valid`
        (`/Game/InStudio/Blueprints/Components/AC_Interactable.Interact` _currentinteractable (`self.OwnerController`))))))