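; AC_BodyPartsHealth is an actor component that gives its owner per-body-part damage and death handling.
; On BeginPlay it registers the owner's AC_SM_BodyPart components with their part data and binds to the owner's point damage event.
; Hits on those components are forwarded to the struck part's TakeDamage.
; When that returns true, a Core part fires OnDeath, while Limb and Weak Spot parts are severed using the hit's direction, location and bone.
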(event `self.ReceiveBeginPlay`
  (`|ExecutionSequence`
    (:`then_0`
      (for _array_element (`Actor.K2_GetComponentsByClass` (`self.GetOwner`) "/Game/InStudio/Blueprints/Components/AC_SM_BodyPart.AC_SM_BodyPart_C")
        (bind _partdata (`/Game/InStudio/Blueprints/Components/AC_SM_BodyPart.GetPartData` _array_element))
        (`BlueprintMapLibrary.Map_Add` (`self.BodyParts`) _array_element _partdata)))
    (:`then_1`
      (add `Actor.OnTakePointDamage` (`self.GetOwner`) (delegate `OnTakePointDamage_Event`)))))

(event `OnTakePointDamage_Event`
  (params (DamagedActor :type "Actor Object Reference") (Damage :type "Float (single-precision)") (InstigatedBy :type "Controller Object Reference") (HitLocation :type "Vector Structure") (FHitComponent :type "PrimitiveComponent Object Reference") (BoneName :type Name) (ShotFromDirection :type "Vector Structure") (DamageType :type "DamageType Object Reference") (DamageCauser :type "Actor Object Reference"))
  (bind _asac_sm_body_part (cast `/Game/InStudio/Blueprints/Components/AC_SM_BodyPart` FHitComponent))
  (bind _isdead (`/Game/InStudio/Blueprints/Components/AC_SM_BodyPart.TakeDamage` _asac_sm_body_part Damage))
  (if _isdead
    (bind _partdata (`/Game/InStudio/Blueprints/Components/AC_SM_BodyPart.GetPartData` _asac_sm_body_part))
    (switch `/Game/InStudio/Blueprints/Data/E_BodyPartTypes` (`.BodyPartType_14_B252B0794059528096A444ABF2E970FC` (break `/Game/InStudio/Blueprints/Data/S_BodyPartData` _partdata))
      (:`NewEnumerator2`
        (`self.OnDeath`))
      (:`NewEnumerator1`
        (`/Game/InStudio/Blueprints/Components/AC_SM_BodyPart.SevereLimb` _asac_sm_body_part ShotFromDirection HitLocation BoneName :!label _label))
      (:`NewEnumerator0`
        (goto _label)))))