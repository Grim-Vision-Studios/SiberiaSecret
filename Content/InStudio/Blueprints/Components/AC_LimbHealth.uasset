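; Actor component that gives a skeletal mesh destructible weak and crit hit points with their own health.
; SpawnHitCollison attaches tagged sphere components to bones of the mesh set by SetMeshTarget, storing their health in a map.
; The owner's point damage event reduces the struck sphere's health, destroying it at zero and printing the result.
; In Debug mode, Tick uses zero-length sphere traces to draw each sphere colored by tag.
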(event `self.ReceiveBeginPlay`
  (add `Actor.OnTakePointDamage` (`self.GetOwner`) (delegate `OnTakePointDamage_Event`)))

(event `OnTakePointDamage_Event`
  (params (DamagedActor :type "Actor Object Reference") (Damage :type "Float (single-precision)") (InstigatedBy :type "Controller Object Reference") (HitLocation :type "Vector Structure") (FHitComponent :type "PrimitiveComponent Object Reference") (BoneName :type Name) (ShotFromDirection :type "Vector Structure") (DamageType :type "DamageType Object Reference") (DamageCauser :type "Actor Object Reference"))
  (bind _assphere_collision (cast `SphereComponent` FHitComponent))
  (if (`BlueprintMapLibrary.Map_Contains` (`self.SpawnedHitPoints`) _assphere_collision)
    (`self.DamageHitPoint` _assphere_collision Damage)))

(event `SpawnHitCollison`
  (`/Engine/EditorBlueprintResources/StandardMacros.IsValid` (`self.OwnerMesh`)
    (:`Is Valid`
      (`|ExecutionSequence`
        (:`then_0`
          (for _array_element (`self.WeakPoints`)
            (`self.AddHitPoint` _array_element)))
        (:`then_1`
          (for _array_element_2 (`self.CritPoints`)
            (`self.AddHitPoint` _array_element_2 "Crit")))))))

(event `self.ReceiveTick`
  (params (DeltaSeconds :type "Float (single-precision)"))
  (if (`self.Debug`)
    (bind _keys (`BlueprintMapLibrary.Map_Keys` (`self.SpawnedHitPoints`)))
    (for _array_element _keys
      (switch `name` (`|GetArrayItem` (`ActorComponent.ComponentTags` _array_element))
        (:`Weak`
          (`self.TraceHitPointDebug` _array_element (struct :`R` 0.942708 :`G` 0.728194 :`B` 0.005077 :`A` 1.0)))
        (:`Crit`
          (`self.TraceHitPointDebug` _array_element (struct :`R` 1.0 :`G` 0.026519 :`A` 1.0)))))))

(fn `AddHitPoint`
  (params (HitPointData :type "/Game/InStudio/Blueprints/Data/Stucts/S_HitPoint Structure") (PointTag :type Name :default "Weak"))
  (bind ((`Radius_18_4647B2E145C7AB7C0CC76F80F520577E` _radius) (`Health_20_0137FE5A4BB97E6401B30CB29E6B6E51` _health)) (break `/Game/InStudio/Blueprints/Data/Stucts/S_HitPoint` HitPointData))
  (bind _returnvalue (`|AddComponentByClass` (`self.GetOwner`) "/Script/Engine.SphereComponent" true (`KismetMathLibrary.MakeTransform` (0.0 0.0 0.0))))
  (`SceneComponent.K2_AttachToComponent` _returnvalue (`self.OwnerMesh`) (`.Bone_21_B252B0794059528096A444ABF2E970FC` (break `/Game/InStudio/Blueprints/Data/Stucts/S_HitPoint` HitPointData)) "SnapToTarget" "SnapToTarget" "KeepRelative" true)
  (`SphereComponent.SetSphereRadius` _returnvalue _radius true)
  (`BlueprintMapLibrary.Map_Add` (`self.SpawnedHitPoints`) _returnvalue (make `/Game/InStudio/Blueprints/Data/Stucts/S_Health` _health _health))
  (`KismetArrayLibrary.Array_Add` (`ActorComponent.ComponentTags` _returnvalue) (`local.PointTag`)))

(fn `DamageHitPoint`
  (params (HitPoint :type "SphereComponent Object Reference (by ref)") (Damage :type "Float (single-precision)"))
  (bind _value (`BlueprintMapLibrary.Map_Find` (`self.SpawnedHitPoints`) HitPoint))
  (bind ((`MaxHealth_4_E0DDB8B74CCC001B06C8679B379810B5` _maxhealth)) (break `/Game/InStudio/Blueprints/Data/Stucts/S_Health` _value))
  (bind _returnvalue (`KismetMathLibrary.FClamp` (- (`.CurrentHealth_6_A0147AC94F00ADD9D666ACBA8F6775AF` (break `/Game/InStudio/Blueprints/Data/Stucts/S_Health` _value)) Damage) 0.0 _maxhealth))
  (`BlueprintMapLibrary.Map_Add` (`self.SpawnedHitPoints`) (`local.HitPoint`) (make `/Game/InStudio/Blueprints/Data/Stucts/S_Health` _maxhealth _returnvalue))
  (if (== _returnvalue 0.0)
    (`self.DestroyHitPoint` (`local.HitPoint`))
    (else
      (`KismetSystemLibrary.PrintString` (`KismetStringLibrary.Concat_StrStr` (`KismetSystemLibrary.GetDisplayName` (`local.HitPoint`)) " Was Hit")))))

(fn `DestroyHitPoint`
  (params (HitPoint :type "SphereComponent Object Reference"))
  (`BlueprintMapLibrary.Map_Remove` (`self.SpawnedHitPoints`) HitPoint)
  (`self.K2_DestroyComponent` HitPoint)
  (`KismetSystemLibrary.PrintString` (`KismetStringLibrary.Concat_StrStr` (`KismetSystemLibrary.GetDisplayName` HitPoint) " Was Destoryed")))

(fn `SetMeshTarget`
  (params (`Skeletal Mesh` :type "SkeletalMeshComponent Object Reference"))
  (set `self.OwnerMesh` `Skeletal Mesh`))

(fn `TraceHitPointDebug`
  (params (HitPointCollision :type "SphereComponent Object Reference") (TraceColor :type "LinearColor Structure"))
  (bind _returnvalue (`SceneComponent.K2_GetComponentLocation` HitPointCollision))
  (`KismetSystemLibrary.SphereTraceMulti` _returnvalue _returnvalue (`SphereComponent.GetUnscaledSphereRadius` HitPointCollision) "TraceTypeQuery1" false (`|MakeArray` (`self.GetOwner`)) "ForOneFrame" true TraceColor))