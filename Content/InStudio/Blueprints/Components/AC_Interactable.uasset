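; Actor component that makes its owning actor interactable, with a lock that can block the interaction.
; On BeginPlay it caches the owner's AC_InteractWidget component if one exists.
; Interact fires the success dispatcher, clears IsReady and hides the widget's interact message when unlocked, or only fires the failure dispatcher when locked.
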(event `self.ReceiveBeginPlay`
  (bind _returnvalue (`Actor.GetComponentByClass` (`self.GetOwner`) "/Game/InStudio/Blueprints/Components/AC_InteractWidget.AC_InteractWidget_C"))
  (`/Engine/EditorBlueprintResources/StandardMacros.IsValid` _returnvalue
    (:`Is Valid`
      (set `self.InteractWidget` _returnvalue))))

(event `Interact`
  (if (not (`self.IsLocked`))
    (`self.OnInteractSuccess` null)
    (set `self.IsReady` false)
    (`/Game/InStudio/Blueprints/Components/AC_InteractWidget.HideInteractMessage` (`self.InteractWidget`))
    (else
      (`self.OnInteractFailed` null))))