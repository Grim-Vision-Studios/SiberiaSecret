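; Actor component that manages its owner's stored weapon slots and the weapon held in the first-person hand.
; Equipping removes the held weapon, async-loads the slot's soft class, spawns it with saved upgrades and attaches it to the "RArm"-tagged mesh.
; Adding fills the first empty slot; add, remove and upgrade edits refresh the held weapon when its slot changes.
; Dispatchers announce equips, unequips, additions and upgrade updates.
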(event `EquipWeapon`
  (params (Slot :type Integer))
  (bind _returnvalue (`self.GetOwner`))
  (bind (_output_name _output_description _output_icon _output_weaponclass _output_upgrades) (break `/Game/InStudio/Blueprints/Data/S_WeaponData` (`|GetArrayItem` (`self.StoredWeapons`) Slot)))
  (`/Engine/EditorBlueprintResources/StandardMacros.IsValid` (`self.HeldWeapon`)
    (:`Is Valid`
      ;[1 1 1] Remove Previous Weapon
      (`self.UnEquipWeapon`))
    (:`Is Not Valid`
      _))
  (if (`KismetSystemLibrary.IsValidSoftClassReference` _output_weaponclass)
    ;[1 1 1] Spawn Equipped Weapon
    (bind _class (`|LoadAssetClass` _output_weaponclass)
      (:`Completed`
        (bind _asbp_weapon_base (castclass `/Game/InStudio/Blueprints/Weapons/BP_Weapon_Base` _class))
        (bind _returnvalue_2 (`|SpawnActorFromClass` _asbp_weapon_base (`KismetMathLibrary.MakeTransform` (0.0 0.0 0.0)) "Undefined" "OverrideRootScale" _returnvalue (cast `Character` _returnvalue :!pure true)))
        (bind _output_get (set `self.HeldWeapon` _returnvalue_2))
        ;[1 1 1] Apply Saved Upgrades
        (`/Game/InStudio/Blueprints/Weapons/BP_Weapon_Base.ApplyUpgrades` _output_get _output_upgrades)
        ;[1 1 1] Hide Weapon Shadow In First Person Hand
        (`PrimitiveComponent.SetCastShadow` (`/Game/InStudio/Blueprints/Weapons/BP_Weapon_Base.WeaponHilt` (`self.HeldWeapon`)) false)
        (`PrimitiveComponent.SetCastShadow` (`/Game/InStudio/Blueprints/Weapons/BP_Weapon_Base.WeaponTop` (`self.HeldWeapon`)) false)
        ;[1 1 1] Attach To Player
        (`Actor.K2_AttachToComponent` (`self.HeldWeapon`) (`|GetArrayItem` (`Actor.GetComponentsByTag` (`self.GetOwner`) "/Script/Engine.SkeletalMeshComponent" "RArm")) "WeaponGrip" "SnapToTarget" "SnapToTarget" "KeepRelative" true)
        ;[1 1 1] Send Equipped Dispatcher Message
        (`self.OnEquipped` (`self.HeldWeapon`))))))

(fn `AddWeapon`
  (params (NewWeaponData :type "/Game/InStudio/Blueprints/Data/S_WeaponData Structure"))
  (locals (NewData :type "/Game/InStudio/Blueprints/Data/S_WeaponData Structure") (AlteredIndex :type Integer :default -1))
  (bind _alteredindex (`local.AlteredIndex`))
  (bind _alteredindex_2 (`local.AlteredIndex`))
  (bind _storedweapons (`self.StoredWeapons`))
  (set `local.NewData` NewWeaponData)
  ;[1 1 1] Find Next Open Slot
  (for (_array_element _array_index) (`self.StoredWeapons`)
    (if (not (`KismetSystemLibrary.IsValidSoftClassReference` (`.WeaponClass_94_56F02D16443CF72713514C97E9A80AEC` (break `/Game/InStudio/Blueprints/Data/S_WeaponData` _array_element))))
      (set `local.AlteredIndex` _array_index)
      (break)))
  ;[1 1 1] Check If Slot Was Found
  (if (`KismetArrayLibrary.Array_IsValidIndex` (`self.StoredWeapons`) _alteredindex)
    ;[1 1 1] Add new weapon data and call updated
    (`KismetArrayLibrary.Array_Set` _storedweapons _alteredindex (`local.NewData`))
    (`self.OnStoredWeaponUpdated` (`|GetArrayItem` _storedweapons _alteredindex_2) _alteredindex_2)
    ;[1 1 1] Re-equip weapon if changed weapon is held
    (if (== _alteredindex_2 (`self.HeldSlot`))
      (`self.EquipWeapon` (`self.HeldSlot`)))))

(fn `RemoveWeapon`
  (params (Slot :type Integer))
  (locals (NewSlot :type Integer))
  (bind _output_get (set `local.NewSlot` Slot))
  (`KismetArrayLibrary.Array_Set` (`self.StoredWeapons`) _output_get)
  (if (== _output_get (`self.HeldSlot`))
    (`self.UnEquipWeapon`)))

(fn `UnEquipWeapon`
  (`Actor.K2_DestroyActor` (`self.HeldWeapon`))
  (`self.OnUnEquipped`))

(fn `UpdateWeaponUpgrades`
  (params (Slot :type Integer) (Upgrades :type "/Game/InStudio/Blueprints/Data/S_WeaponUpgrades Structure"))
  (bind _structout (setmembers `/Game/InStudio/Blueprints/Data/S_WeaponData` :`StructRef` (`|GetArrayItem` (`self.StoredWeapons`) Slot) :`Upgrades` Upgrades))
  (`self.OnStoredWeaponUpdated` _structout Slot)
  (if (== Slot (`self.HeldSlot`))
    (`/Game/InStudio/Blueprints/Weapons/BP_Weapon_Base.ApplyUpgrades` (`self.HeldWeapon`) (`.Upgrades_86_1D1A2EEA461BB829D1110E8FFFC5B543` (break `/Game/InStudio/Blueprints/Data/S_WeaponData` _structout)))))