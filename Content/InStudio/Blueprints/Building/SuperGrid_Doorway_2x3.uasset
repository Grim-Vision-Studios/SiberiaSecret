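; SuperGrid_Doorway_2x3 is a modular doorway building piece with separately materialed external and internal faces.
; Its construction script applies ExternalMaterial to the two external side meshes and the external top, and InternalMaterial to the matching internal set.
; Each material is applied to the first slot only when valid, and the event graph holds no active logic.
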(fn `UserConstructionScript`
  (bind _externalmaterial (`self.ExternalMaterial`))
  (bind _internalmaterial (`self.InternalMaterial`))
  (`|ExecutionSequence`
    (:`then_0`
      (`/Engine/EditorBlueprintResources/StandardMacros.IsValid` _externalmaterial
        (:`Is Valid`
          (`PrimitiveComponent.SetMaterial` (`self.ExternalSide1`) 0 _externalmaterial)
          (`PrimitiveComponent.SetMaterial` (`self.ExternalSide2`) 0 _externalmaterial)
          (`PrimitiveComponent.SetMaterial` (`self.ExternalSideTop`) 0 _externalmaterial))))
    (:`then_1`
      (`/Engine/EditorBlueprintResources/StandardMacros.IsValid` _internalmaterial
        (:`Is Valid`
          (`PrimitiveComponent.SetMaterial` (`self.InternalSide1`) 0 _internalmaterial)
          (`PrimitiveComponent.SetMaterial` (`self.InternalSide2`) 0 _internalmaterial)
          (`PrimitiveComponent.SetMaterial` (`self.InternalSideTop`) 0 _internalmaterial))))))