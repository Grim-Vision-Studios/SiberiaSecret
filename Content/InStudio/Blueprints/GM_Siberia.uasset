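; GM_Siberia is a game mode that manages the player's respawn point and its persistence in a save slot.
; BeginPlay restores the respawn transform from BP_SiberiaSaveGame if a save exists, otherwise it uses the PlayerStart transform.
; SaveGame only updates an existing save, as it never creates a save object.
; DeleteSave clears a hardcoded slot rather than the CurrSaveName slot used elsewhere.
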(event `self.ReceiveBeginPlay`
  (bind _returnvalue (`GameplayStatics.DoesSaveGameExist` (`self.CurrSaveName`)))
  (if _returnvalue
    (`self.LoadGame`)
    (else
      (bind _returnvalue_2 (`GameplayStatics.GetActorOfClass` "/Script/Engine.PlayerStart"))
      (set `self.PlayerRespawnPoint` (`self.GetTransform` _returnvalue_2)))))

(event `LoadGame`
  (bind _returnvalue (`GameplayStatics.LoadGameFromSlot` (`self.CurrSaveName`)))
  (bind _asbp_siberia_save_game (cast `/Game/InStudio/Blueprints/BP_SiberiaSaveGame` _returnvalue))
  (set `self.PlayerRespawnPoint` (`/Game/InStudio/Blueprints/BP_SiberiaSaveGame.RespawnTransform` _asbp_siberia_save_game)))

(event `SaveGame`
  (bind _returnvalue (`GameplayStatics.LoadGameFromSlot` (`self.CurrSaveName`)))
  (bind _asbp_siberia_save_game (cast `/Game/InStudio/Blueprints/BP_SiberiaSaveGame` _returnvalue))
  (set `/Game/InStudio/Blueprints/BP_SiberiaSaveGame.RespawnTransform` (`self.PlayerRespawnPoint`) _asbp_siberia_save_game)
  (`GameplayStatics.SaveGameToSlot` _returnvalue (`self.CurrSaveName`)))

(event `DeleteSave`
  (`GameplayStatics.DeleteGameInSlot` "Save1"))

(fn `UserConstructionScript`)