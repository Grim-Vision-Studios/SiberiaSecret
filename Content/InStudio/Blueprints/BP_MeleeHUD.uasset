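; BP_MeleeHUD is the player HUD that creates the W_PlayerHud widget and manages its weapon wheel.
; On BeginPlay it fills the wheel icons from the weapons stored in the pawn's AC_WepHolder component, then binds to that component's update event to refresh single slots.
; SetWeaponWheelVisability shows or hides the wheel, switching the character between UIOpen and Idle states and centering the mouse when shown.
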(event `self.ReceiveBeginPlay`
  ;[1 1 1] Create Aim Wiget
  (bind _returnvalue (`|CreateWidget` "/Game/InStudio/Art/UI/W_PlayerHud.W_PlayerHud_C" (`GameplayStatics.GetPlayerController` 0)))
  (bind _output_get (set `self.HUDWidget` _returnvalue))
  (`UserWidget.AddToViewport` _output_get 0)
  (`|CreateWidget` "/Game/InStudio/Art/UI/W_PlayerHud.W_PlayerHud_C" (`GameplayStatics.GetPlayerController` 0))
  ;[1 1 1] Save Reference To Weapon Holder
  (bind _output_get_2 (set `self.PlayerWeaponHolder` (`self.GetComponentByClass` (`Controller.K2_GetPawn` (`self.PlayerOwner`)) "/Game/InStudio/Blueprints/Components/AC_WepHolder.AC_WepHolder_C")))
  ;[1 1 1] Initialize Weapon Icons
  (for (_array_element _array_index) (`/Game/InStudio/Blueprints/Components/AC_WepHolder.StoredWeapons` _output_get_2)
    (set `/Game/InStudio/Art/UI/W_AdvancedButton.Image` (make `SlateBrush` "Image" "NoTile" "NoMirror" (32.0 32.0) (struct) (struct :`SpecifiedColor` (struct :`R` 1.0 :`G` 1.0 :`B` 1.0 :`A` 1.0) :`ColorUseRule` "UseColor_Specified") (struct :`CornerRadii` (struct :`W` 1.0) :`Color` (struct :`SpecifiedColor` (struct) :`ColorUseRule` "UseColor_Specified") :`RoundingType` "HalfHeightRadius") (`.Icon_92_82E237B246E162498B5F2C8F32C07E9B` (break `/Game/InStudio/Blueprints/Data/S_WeaponData` _array_element))) (`|GetArrayItem` (`/Game/InStudio/Art/UI/W_WeaponWheel.WeaponWidgets` (`/Game/InStudio/Art/UI/W_PlayerHud.W_WeaponWheel` (`self.HUDWidget`))) _array_index)))
  ;[1 1 1] Update Icons When Stored Weapons Are Updated
  (add `/Game/InStudio/Blueprints/Components/AC_WepHolder.OnStoredWeaponUpdated` (`self.PlayerWeaponHolder`) (delegate `UpdateWeaponWidget`)))

(event `UpdateWeaponWidget`
  (params (NewWeaponData :type "/Game/InStudio/Blueprints/Data/S_WeaponData Structure") (Index :type Integer))
  ;[1 1 1] Update Icons When Stored Weapons Are Updated
  (set `/Game/InStudio/Art/UI/W_AdvancedButton.Image` (make `SlateBrush` "Image" "NoTile" "NoMirror" (32.0 32.0) (struct) (struct :`SpecifiedColor` (struct :`R` 1.0 :`G` 1.0 :`B` 1.0 :`A` 1.0) :`ColorUseRule` "UseColor_Specified") (struct :`CornerRadii` (struct :`W` 1.0) :`Color` (struct :`SpecifiedColor` (struct) :`ColorUseRule` "UseColor_Specified") :`RoundingType` "HalfHeightRadius") (`.Icon_92_82E237B246E162498B5F2C8F32C07E9B` (break `/Game/InStudio/Blueprints/Data/S_WeaponData` NewWeaponData))) (`|GetArrayItem` (`/Game/InStudio/Art/UI/W_WeaponWheel.WeaponWidgets` (`/Game/InStudio/Art/UI/W_PlayerHud.W_WeaponWheel` (`self.HUDWidget`))) Index)))

(fn `SetWeaponWheelVisability`
  (params (NewVisibility :type "ESlateVisibility Enum" :default "Visible"))
  (bind _returnvalue (`GameplayStatics.GetPlayerCharacter` 0))
  (`Widget.SetVisibility` (`/Game/InStudio/Art/UI/W_PlayerHud.W_WeaponWheel` (`self.HUDWidget`)) NewVisibility)
  (switch `ESlateVisibility` NewVisibility
    (:`Visible`
      (message `/Game/InStudio/Blueprints/Interfaces/I_Actions.SwitchState` _returnvalue (struct :`TagName` "Actions.UIOpen"))
      (`/Game/InStudio/Art/UI/W_PlayerHud.CenterMouse` (`self.HUDWidget`)))
    (:`Hidden`
      (message `/Game/InStudio/Blueprints/Interfaces/I_Actions.SwitchState` _returnvalue (struct :`TagName` "Actions.Idle")))))

(fn `UserConstructionScript`)