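; Base character Blueprint for entities, providing sprint, attack and weapon-switch actions on top of a gameplay-tag state machine.
; BeginPlay caches the torso's melee anim instance, and sprint toggles max walk speed between walk and sprint values.
; Attack and weapon switch change state only from Idle, while SwitchState forwards any requested state directly.
; Weapon pickup and starting-weapon setup are stubs, with the WeaponHolder AddWeapon call left unwired.
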(event `self.ReceiveBeginPlay`
  (bind _asam_fpmelee (cast `/Game/InStudio/Art/TempCharacter/Animations/AM_FPMelee` (`SkeletalMeshComponent.GetAnimInstance` (`self.BPC_BodyPart_Torso`))))
  (set `self.AnimInstance` _asam_fpmelee)
  (if (`KismetSystemLibrary.IsValidClass` (`self.StartingWeapon`))
    _))

(event `TrySprint`
  (params (On :type Boolean))
  (bind _charactermovement (`self.CharacterMovement`))
  ;[1 1 1] Sprint
  (if On
    (set `CharacterMovementComponent.MaxWalkSpeed` (`self.Sprint Speed`) _charactermovement)
    (else
      (set `CharacterMovementComponent.MaxWalkSpeed` (`self.Walk Speed`) _charactermovement))))

(event `TryAttack`
  (bind _statemachine (`self.StateMachine`))
  ;[1 1 1] Attack
  (bind _anymatch (`/Game/InStudio/Blueprints/Components/AC_StateMachine.IsCurrentState` _statemachine (`BlueprintGameplayTagLibrary.MakeLiteralGameplayTagContainer` (struct :`GameplayTags` (struct :`(TagName` "Actions.Idle") :`(TagName` "Actions.Attack.End")))) true))
  (if _anymatch
    (`/Game/InStudio/Blueprints/Components/AC_StateMachine.SwitchState` _statemachine (struct :`TagName` "Actions.Attack.Start"))))

(event `/Game/InStudio/Blueprints/Interfaces/I_Actions.SwitchState`
  (params (NewParam :type "GameplayTag Structure"))
  (`/Game/InStudio/Blueprints/Components/AC_StateMachine.SwitchState` (`self.StateMachine`) NewParam))

(event `SwitchWeapon`
  (bind _statemachine (`self.StateMachine`))
  ;[1 1 1] Switch Weapon
  (bind _anymatch (`/Game/InStudio/Blueprints/Components/AC_StateMachine.IsCurrentState` _statemachine (`BlueprintGameplayTagLibrary.MakeLiteralGameplayTagContainer` (struct :`GameplayTags` (struct :`(TagName` "Actions.Idle") :`(TagName` "Actions.Run")))) true))
  (if _anymatch
    (`/Game/InStudio/Blueprints/Components/AC_StateMachine.SwitchState` _statemachine (struct :`TagName` "Actions.SwitchWeapon"))))

(event `self.PickUpWeapon`
  (params (Weapon :type "/Game/InStudio/Blueprints/Data/S_WeaponData Structure"))
  ;[1 1 1] PickUpWeapon
)

(fn `GetCharacterStatus`
  (returns (CharacterState :type "GameplayTag Structure"))
  (return (`/Game/InStudio/Blueprints/Components/AC_StateMachine.CurrentState` (`self.StateMachine`))))

(fn `UserConstructionScript`
  (locals (CurrentComponent :type "SkeletalMeshComponent Object Reference") (CurrentBodyPart :type "/Game/InStudio/Blueprints/Data/S_BodyPartData Structure")))