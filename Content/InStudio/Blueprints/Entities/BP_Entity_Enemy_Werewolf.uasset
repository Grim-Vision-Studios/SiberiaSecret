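; Werewolf enemy entity Blueprint that holds a reference to the level's combat director.
; On BeginPlay it finds the BP_CombatDirector actor and caches it.
; The PlayerDetection overlap checks for the player character but takes no action, and is noted as removable if detection changes.
; Leftover unconnected nodes for setting blackboard spotted and attack flags and playing the attack montage never run.
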(event `self.ReceiveBeginPlay`
  (bind _returnvalue (`GameplayStatics.GetActorOfClass` "/Game/InStudio/Blueprints/Systems/CombatDirector/BP_CombatDirector.BP_CombatDirector_C"))
  (set `self.CombatDirector` _returnvalue))

(event `self.PlayerDetection.OnComponentBeginOverlap`
  (params (OverlappedComponent :type "PrimitiveComponent Object Reference") (OtherActor :type "Actor Object Reference") (OtherComp :type "PrimitiveComponent Object Reference") (OtherBodyIndex :type Integer) (bFromSweep :type Boolean) (SweepResult :type "HitResult Structure (by ref)"))
  ;[1 1 1] If we change how detection works then this can be removed
  (if (== (`GameplayStatics.GetPlayerCharacter` 0) OtherActor)
    _))

(fn `UserConstructionScript`)