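; Banshee enemy entity that rolls a decision value for its AI through the Blackboard.
; On BeginPlay it binds CreateInt to the RandomInt event and caches a reference to the level's BP_CombatDirector.
; CreateInt writes the Decision key, choosing randomly between two options when "CanAttack?" is true and falling back to the first option otherwise.
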(event `self.ReceiveBeginPlay`
  (add `self.RandomInt` (delegate `CreateInt`))
  (bind _returnvalue (`GameplayStatics.GetActorOfClass` "/Game/InStudio/Blueprints/CombatDirector/BP_CombatDirector.BP_CombatDirector_C"))
  (set `self.CombatDirector` _returnvalue))

(event `CreateInt`
  (bind _returnvalue (`AIBlueprintHelperLibrary.GetBlackboard` null))
  ;[1 1 1] Random Int for Decision making
  (if (`BlackboardComponent.GetValueAsBool` (`AIBlueprintHelperLibrary.GetBlackboard` null) "CanAttack?")
    (`BlackboardComponent.SetValueAsInt` _returnvalue (`self.Decision`) (`KismetMathLibrary.RandomIntegerInRange` 1 2))
    (else
      (`BlackboardComponent.SetValueAsInt` _returnvalue (`self.Decision`) 1))))

(fn `UserConstructionScript`
  (`parent.UserConstructionScript`))