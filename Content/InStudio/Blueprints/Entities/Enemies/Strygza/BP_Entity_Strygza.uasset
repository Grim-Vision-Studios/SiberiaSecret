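; Strygza enemy entity that feeds player detection and randomized decisions into its AI Blackboard.
; A detection overlap flags the player as spotted.
; A bound random-int event writes the Decision key, randomizing it only when attacking is allowed and otherwise using a fixed default.
; A looping test timer shows the enemy's Combat Director grading and attack permission on text renders for debugging.
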(event `test`
  ;[1 1 1] testing
  (for _array_element (`/Game/InStudio/Blueprints/CombatDirector/BP_CombatDirector.EnemyList` (stale `self.ReceiveBeginPlay` _output_get))
    (if (== _array_element self)
      (`TextRenderComponent.K2_SetText` (`self.TextRender`) (`KismetTextLibrary.Conv_DoubleToText` (`BlueprintMapLibrary.Map_Find` (`/Game/InStudio/Blueprints/CombatDirector/BP_CombatDirector.EnemyGrading` (stale `self.ReceiveBeginPlay` _output_get)) _array_element) "HalfToEven"))
      (`TextRenderComponent.K2_SetText` (`self.TextRender1`) (`KismetTextLibrary.Conv_BoolToText` (`BlackboardComponent.GetValueAsBool` (`AIBlueprintHelperLibrary.GetBlackboard` null) "CanAttack?"))))))

(event `self.ReceiveBeginPlay`
  (add `self.RandomInt` (delegate `CreateInt`))
  (bind _returnvalue (`GameplayStatics.GetActorOfClass` "/Game/InStudio/Blueprints/CombatDirector/BP_CombatDirector.BP_CombatDirector_C"))
  (bind _output_get (set `self.CombatDirector` _returnvalue))
  ;[1 1 1] testing
  (`KismetSystemLibrary.K2_SetTimerDelegate` (delegate `test`) 0.1 true))

(event `CreateInt`
  (bind _returnvalue (`AIBlueprintHelperLibrary.GetBlackboard` null))
  ;[1 1 1] Random Int for Decision making
  (if (`BlackboardComponent.GetValueAsBool` (`AIBlueprintHelperLibrary.GetBlackboard` null) "CanAttack?")
    (`BlackboardComponent.SetValueAsInt` _returnvalue (`self.Decision`) (`KismetMathLibrary.RandomIntegerInRange` 1 3))
    (else
      (`BlackboardComponent.SetValueAsInt` _returnvalue (`self.Decision`) 1))))

(event `self.PlayerDetection.OnComponentBeginOverlap`
  (params (OverlappedComponent :type "PrimitiveComponent Object Reference") (OtherActor :type "Actor Object Reference") (OtherComp :type "PrimitiveComponent Object Reference") (OtherBodyIndex :type Integer) (bFromSweep :type Boolean) (SweepResult :type "HitResult Structure (by ref)"))
  ;[1 1 1] When enemy spots player, communicate to blackboard
  (if (== (`GameplayStatics.GetPlayerCharacter` 0) OtherActor)
    (`BlackboardComponent.SetValueAsBool` (`AIBlueprintHelperLibrary.GetBlackboard` null) "PlayerSpotted?" true)))

(fn `UserConstructionScript`)