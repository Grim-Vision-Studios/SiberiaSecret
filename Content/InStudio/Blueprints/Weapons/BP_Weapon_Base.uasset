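; Base weapon actor that holds damage, speed and durability stats for weapons in the game.
; On BeginPlay current durability is set to maximum, and ApplyUpgrades adds each upgrade amount, scaled by a per-stat increase, to its stat.
; Drop detaches the weapon from its actor and teleports it to a given location and rotation if it has a valid owner.
; DamageTrace is a stub that reports no hit.
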(event `self.ReceiveBeginPlay`
  (set `self.CurDur` (`self.MaxDur`)))

(fn `ApplyUpgrades`
  (params (UpgradesToAdd :type "/Game/InStudio/Blueprints/Data/S_WeaponUpgrades Structure"))
  (bind (_damage _speed _maxdur) (break `/Game/InStudio/Blueprints/Data/S_WeaponUpgrades` UpgradesToAdd))
  (`self.UpgradeDamage` _damage)
  (`self.UpgradeSpeed` _speed)
  (`self.UpgradeDurability` _maxdur))

(fn `DamageTrace`
  (returns (HitResult :type "HitResult Structure") (DidHit :type Boolean))
  (return (struct) false))

(fn `Drop`
  (params (Location :type "Vector Structure") (Rotation :type "Rotator Structure"))
  (`/Engine/EditorBlueprintResources/StandardMacros.IsValid` (`self.GetOwner`)
    (:`Is Valid`
      (`self.K2_DetachFromActor` "KeepRelative")
      (`self.K2_SetActorLocationAndRotation` Location Rotation false true))))

(fn `UpgradeDamage`
  (params (Amount :type Integer))
  (set `self.Damage` (+ (* Amount (`self.DamageIncrease`)) (`self.Damage`))))

(fn `UpgradeDurability`
  (params (Amount :type Integer))
  (set `self.MaxDur` (+ (* Amount (`self.DurIncrease`)) (`self.MaxDur`))))

(fn `UpgradeSpeed`
  (params (Amount :type Integer))
  (set `self.Speed` (+ (* Amount (`self.SpeedIncrease`)) (`self.Speed`))))

(fn `UserConstructionScript`)