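; BP_Entity_Enemy_Core is a core enemy entity in the SeverCombat system that sets up the enemy's body parts.
; InitializeBodyParts takes a torso plus head and limb collections, looking up the Torso, Head or Limb row in EntityTable for each.
; Each part whose row is found receives its type, health and armor, then joins the BodyParts list without duplicates.
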(fn `InitializeBodyParts`
  (params (Torso :type "/Game/InStudio/Blueprints/SeverCombat/BPC_BodyPart Object Reference") (Heads :type "Array of /Game/InStudio/Blueprints/SeverCombat/BPC_BodyPart Object Reference") (Limbs :type "Array of /Game/InStudio/Blueprints/SeverCombat/BPC_BodyPart Object Reference"))
  (locals (CurrentComponent :type "/Game/InStudio/Blueprints/SeverCombat/BPC_BodyPart Object Reference"))
  (`|ExecutionSequence`
    (:`then_0`
      (set `local.CurrentComponent` Torso)
      (bind _returnvalue (`|GetDataTableRow` (`self.Entity Table`) "Torso")
        (:`then`
          (bind (_bodyparttype _health _armor) (break `/Game/InStudio/Blueprints/SeverCombat/Data/S_BodyPart` _returnvalue))
          (`/Game/InStudio/Blueprints/SeverCombat/BPC_BodyPart.Set Variables` (`local.CurrentComponent`) _bodyparttype _health _armor)
          (`KismetArrayLibrary.Array_AddUnique` (`self.BodyParts`) (`local.CurrentComponent`) :!label _label))))
    (:`then_1`
      (for _array_element Heads
        (set `local.CurrentComponent` _array_element)
        (bind _returnvalue_2 (`|GetDataTableRow` (`self.Entity Table`) "Head")
          (:`then`
            (bind (_bodyparttype_2 _health_2 _armor_2) (break `/Game/InStudio/Blueprints/SeverCombat/Data/S_BodyPart` _returnvalue_2))
            (`/Game/InStudio/Blueprints/SeverCombat/BPC_BodyPart.Set Variables` (`local.CurrentComponent`) _bodyparttype_2 _health_2 _armor_2)
            (goto _label))))
      (for _array_element_2 Limbs
        (set `local.CurrentComponent` _array_element_2)
        (bind _returnvalue_3 (`|GetDataTableRow` (`self.Entity Table`) "Limb")
          (:`then`
            (bind (_bodyparttype_3 _health_3 _armor_3) (break `/Game/InStudio/Blueprints/SeverCombat/Data/S_BodyPart` _returnvalue_3))
            (`/Game/InStudio/Blueprints/SeverCombat/BPC_BodyPart.Set Variables` (`local.CurrentComponent`) _bodyparttype_3 _health_3 _armor_3)
            (goto _label)))))))

(fn `UserConstructionScript`)