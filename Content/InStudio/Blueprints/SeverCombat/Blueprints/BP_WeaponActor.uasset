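; BP_WeaponActor is a weapon pickup that displays a weapon on a skeletal mesh.
; Its construction script finds the BP_WeaponsMaster actor and uses the WeaponMeshSelect choice to pick an entry from its Weapons array, previewing that mesh on placement.
; SpawnWeapon overrides the stored weapon and mesh at runtime.
; PickUpWeapon destroys the actor and returns the weapon data with an IsWeapon flag.
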(event `/Game/InStudio/Blueprints/SeverCombat/Blueprints/Interfaces/I_Intereactable.SpawnWeapon`
  (params (Weapon :type "/Game/InStudio/Blueprints/SeverCombat/Blueprints/Data/S_Weapon Structure"))
  (bind _output_get (set `self.CurrWeapon` Weapon))
  (`SkinnedMeshComponent.SetSkinnedAssetAndUpdate` (`self.SkeletalMeshComponent`) (`.WeaponMesh_28_260294D146A7DCE78E896FBFAAC568F3` (break `/Game/InStudio/Blueprints/SeverCombat/Blueprints/Data/S_Weapon` _output_get)) true))

(fn `PickUpWeapon`
  (returns (Weapon :type "/Game/InStudio/Blueprints/SeverCombat/Blueprints/Data/S_Weapon Structure") (IsWeapon :type Boolean))
  (`self.K2_DestroyActor`)
  (return (`self.CurrWeapon`) true))

(fn `UserConstructionScript`
  (bind _returnvalue (`GameplayStatics.GetActorOfClass` "/Game/InStudio/Blueprints/SeverCombat/Blueprints/BP_WeaponsMaster.BP_WeaponsMaster_C"))
  (bind _output_get (set `self.WeaponMaster` _returnvalue))
  (bind _output_get_2 (set `self.CurrWeapon` (`|GetArrayItem` (`/Game/InStudio/Blueprints/SeverCombat/Blueprints/BP_WeaponsMaster.Weapons` _output_get) (select `/Game/InStudio/Blueprints/SeverCombat/Blueprints/Data/E_WeaponNames` (`self.WeaponMeshSelect`) :`NewEnumerator0` 1 :`NewEnumerator1` 2 :`NewEnumerator2` 3))))
  (`SkinnedMeshComponent.SetSkinnedAssetAndUpdate` (`self.SkeletalMeshComponent`) (`.WeaponMesh_28_260294D146A7DCE78E896FBFAAC568F3` (break `/Game/InStudio/Blueprints/SeverCombat/Blueprints/Data/S_Weapon` _output_get_2)) true))