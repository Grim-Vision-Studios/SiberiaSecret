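; Base character Blueprint for SeverCombat entities, providing sprint toggle, attack, kick, block and weapon switching.
; A shared IsBusy flag gates attack, block and switch; attack and kick also disable movement.
; Switching messages the torso AnimInstance and the Weapon, while GetCharacterStatus reports action flags and armed state, with fixed prepared and aim values.
; EditWeapon, GetWeapon and SetWeapon are empty stubs.
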(event `Sprint`
  (bind _charactermovement (`self.CharacterMovement`))
  ;[1 1 1] Sprint
  (`/Engine/EditorBlueprintResources/StandardMacros.FlipFlop`
    (:`A`
      (set `CharacterMovementComponent.MaxWalkSpeed` (`self.Sprint Speed`) _charactermovement))
    (:`B`
      (set `CharacterMovementComponent.MaxWalkSpeed` (`self.Walk Speed`) _charactermovement))))

(event `Attack`
  ;[1 1 1] Attack
  (if (not (`self.IsBusy`))
    (bind _output_get (set `self.IsAttacking` true))
    (set `self.IsBusy` _output_get)
    (`CharacterMovementComponent.DisableMovement` (`self.CharacterMovement`))))

(event `StartKick`
  ;[1 1 1] Kick
  (bind _output_get (set `self.IsKicking` true))
  (set `self.IsBusy` _output_get)
  (`CharacterMovementComponent.DisableMovement` (`self.CharacterMovement`)))

(event `/Game/InStudio/Blueprints/SeverCombat/Blueprints/Interfaces/I_Combat.Kick`
  ;[1 1 1] Kick
  (bind _output_get (set `self.IsKicking` false))
  (set `self.IsBusy` _output_get))

(event `/Game/InStudio/Blueprints/SeverCombat/Blueprints/Interfaces/I_Combat.DeactivateAim`
  ;[1 1 1] Attack
  (bind _output_get (set `self.IsAttacking` false))
  (set `self.IsBusy` _output_get))

(event `Block`
  (params (IsPressed :type Boolean))
  ;[1 1 1] Block
  (if (`self.IsBusy`)
    _
    (elif IsPressed
      (bind _output_get (set `self.IsBlocking` true))
      (set `self.IsBusy` _output_get)
      (else
        (bind _output_get_2 (set `self.IsBlocking` false))
        (set `self.IsBusy` _output_get_2)))))

(event `Switch Weapon`
  ;[1 1 1] Switch Weapon
  (if (not (`self.IsBusy`))
    (bind _output_get (set `self.isSwitching` true))
    (set `self.IsBusy` _output_get)
    (message `/Game/InStudio/Blueprints/SeverCombat/Blueprints/Interfaces/I_Combat.SwitchWeapon` (`SkeletalMeshComponent.GetAnimInstance` (`self.BPC_BodyPart_Torso`)))
    (`/Game/InStudio/Blueprints/SeverCombat/Blueprints/BP_WepHolder.Switch Weapon` (`self.Weapon`))))

(fn `Edit Weapon`
  (params (CurrWeapon :type "/Game/InStudio/Blueprints/SeverCombat/Blueprints/Data/S_Weapon Structure") (EditType :type "/Game/InStudio/Blueprints/SeverCombat/Blueprints/Data/E_Upgrades Enum" :default "NewEnumerator0"))
  (returns (UpgradedWeapon :type "/Game/InStudio/Blueprints/SeverCombat/Blueprints/Data/S_Weapon Structure"))
  (return))

(fn `GetCharacterStatus`
  (returns (HasWeapon :type Boolean) (IsAttacking :type Boolean) (IsBlocking :type Boolean) (IsKicking :type Boolean) (isPrepared :type Boolean) (AimDirection :type "/Game/InStudio/Blueprints/SeverCombat/Blueprints/Data/E_AimDirection Enum"))
  (if (!= (`.Index_31_9DE60E67468BFA8216A140B084BAFE3B` (break `/Game/InStudio/Blueprints/SeverCombat/Blueprints/Data/S_Weapon` (`/Game/InStudio/Blueprints/SeverCombat/Blueprints/BP_WepHolder.CurrWeapon` (`self.Weapon`)))) 0)
    (set `self.HasWeapon` true)
    (else
      (bind _output_get (set `self.HasWeapon` false))))
  (return _output_get (`self.IsAttacking`) (`self.IsBlocking`) (`self.IsKicking`) true "NewEnumerator0"))

(fn `GetWeapon`
  (returns (CurWeapon :type "/Game/InStudio/Blueprints/SeverCombat/Blueprints/Data/S_Weapon Structure"))
  (return))

(fn `SetWeapon`
  (params (WeaponIndex :type Integer))
  (returns (NewCurrWeapon :type "/Game/InStudio/Blueprints/SeverCombat/Blueprints/Data/S_Weapon Structure"))
  (return))

(fn `UserConstructionScript`
  (locals (CurrentComponent :type "SkeletalMeshComponent Object Reference") (CurrentBodyPart :type "/Game/InStudio/Blueprints/SeverCombat/Blueprints/Data/S_BodyPart Structure")))