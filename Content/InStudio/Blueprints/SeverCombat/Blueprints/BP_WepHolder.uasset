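; BP_WepHolder tracks a current and a stored weapon for whatever holds weapons in the SeverCombat system.
; On BeginPlay it finds the level's BP_WeaponsMaster, printing a warning if none exists, and takes the first weapon entry as the default.
; Dropping a non-default weapon messages the master with its location and rotation, then reverts to that default.
; SwitchWeapon swaps the current and stored weapons.
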(event `self.ReceiveBeginPlay`
  (bind _returnvalue (`GameplayStatics.GetActorOfClass` "/Game/InStudio/Blueprints/SeverCombat/Blueprints/BP_WeaponsMaster.BP_WeaponsMaster_C"))
  (`/Engine/EditorBlueprintResources/StandardMacros.IsValid` _returnvalue
    (:`Is Valid`
      (bind _output_get (set `self.WeaponMaster` _returnvalue))
      (set `self.CurrWeapon` (`|GetArrayItem` (`/Game/InStudio/Blueprints/SeverCombat/Blueprints/BP_WeaponsMaster.Weapons` _output_get))))
    (:`Is Not Valid`
      (`KismetSystemLibrary.PrintString` "No Weapon Master Actor Present in Level"))))

(event `Drop Curr Weapon`
  (params (Location :type "Vector Structure") (Rotation :type "Rotator Structure"))
  (bind (_currweapon_weaponname _currweapon_weaponmesh _currweapon_index) (break `/Game/InStudio/Blueprints/SeverCombat/Blueprints/Data/S_Weapon` (`self.CurrWeapon`)))
  (if (!= _currweapon_index 0)
    (message `/Game/InStudio/Blueprints/SeverCombat/Blueprints/Interfaces/I_Combat.Drop Weapon` (`self.WeaponMaster`) (`self.CurrWeapon`) Location Rotation)
    (set `self.CurrWeapon` (`|GetArrayItem` (`/Game/InStudio/Blueprints/SeverCombat/Blueprints/BP_WeaponsMaster.Weapons` (`self.WeaponMaster`))))))

(event `Switch Weapon`
  (set `self.SaveWep` (`self.CurrWeapon`))
  (set `self.CurrWeapon` (`self.StoredWeapon`))
  (set `self.StoredWeapon` (`self.SaveWep`)))