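; Weapon pickup that shows an attached weapon actor and adds that weapon to the player's stored weapons on interaction.
; On BeginPlay it looks up the attached weapon's row in DT_Weapons, while a SpawnWeapon event can replace the display actor with one attached to WeaponRoot.
; Interacting passes the data to AC_WepHolder, sends a HUD collection notice, destroys the display weapon and disables PickupRange collision.
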(event `self.ReceiveBeginPlay`
  ;[1 1 1] Collect Weapon Reference Data
  (bind _asbp_weapon_base (cast `/Game/InStudio/Blueprints/Weapons/BP_Weapon_Base` (`|GetArrayItem` (`self.GetAttachedActors` true))))
  (bind _returnvalue (`|GetDataTableRow` "/Game/InStudio/Blueprints/Data/DataTables/DT_Weapons.DT_Weapons" (`/Game/InStudio/Blueprints/Weapons/BP_Weapon_Base.RowName` _asbp_weapon_base))
    (:`then`
      (set `self.WeaponData` _returnvalue))))

(event `SpawnWeapon`
  (bind _output (`|GetArrayItem` (`self.GetAttachedActors` true)))
  ;[1 1 1] Spawn Weapon Reference
  (`/Engine/EditorBlueprintResources/StandardMacros.IsValid` _output
    (:`Is Valid`
      (`self.K2_DestroyActor` _output))
    (:`Is Not Valid`
      _))
  (bind _returnvalue (`|SpawnActorFromClass` (`self.Weapon`) (`KismetMathLibrary.MakeTransform` (0.0 0.0 0.0)) "Undefined" "SelectDefaultAtRuntime" null null))
  (`self.K2_AttachToComponent` _returnvalue (`self.WeaponRoot`) "None" "SnapToTarget" "KeepWorld" "KeepRelative" true))

(event `self.AC_Interactable.OnInteracted`
  (bind (_name _description _icon) (break `/Game/InStudio/Blueprints/Data/S_ItemData` (`self.WeaponData`)))
  ;[1 1 1] Add Weapon To Player Stored Weapons
  (`/Game/InStudio/Blueprints/Components/AC_WepHolder.AddWeapon` (`self.GetComponentByClass` (`GameplayStatics.GetPlayerCharacter` 0) "/Game/InStudio/Blueprints/Components/AC_WepHolder.AC_WepHolder_C") (`self.WeaponData`))
  ;[1 1 1] Send Notif To Player Regarding Weapon Collected
  (message `/Game/InStudio/Blueprints/Interfaces/I_Hud.SendImportantInfo` (`PlayerController.GetHUD` (`GameplayStatics.GetPlayerController` 0)) (`KismetTextLibrary.Conv_StringToText` (`KismetStringLibrary.Concat_StrStr` (`KismetTextLibrary.Conv_TextToString` _name) " Collected")) _icon)
  ;[1 1 1] Destroy Weapon Reference & Disable Interact Collision
  (`self.K2_DestroyActor` (cast `/Game/InStudio/Blueprints/Weapons/BP_Weapon_Base` (`|GetArrayItem` (`self.GetAttachedActors` true)) :!pure true))
  (`PrimitiveComponent.SetCollisionEnabled` (`self.PickupRange`) "NoCollision"))

(fn `UserConstructionScript`
  (`parent.UserConstructionScript`))