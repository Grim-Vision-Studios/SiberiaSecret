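; BPC_StateMachine is an actor component, going by its prefix, that runs a simple state machine with Gameplay Tags as states.
; SwitchState starts the initial state on BeginPlay, rejects empty or already active tags, and otherwise ends the old state, initializes the new one and announces the change.
; Init, Tick and End are forwarded through delegates, leaving state logic to listeners.
; IsCurrentState tests the active tag against a container.
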(event `self.ReceiveBeginPlay`
  (`self.SwitchState` (`self.InitialState`)))

(event `self.ReceiveTick`
  (params (DeltaSeconds :type "Float (single-precision)"))
  (if (`self.CanTick`)
    (`self.TickState` DeltaSeconds)))

(fn `EndState`
  (`self.EndStateDelagate` (`self.CurrentState`)))

(fn `InitState`
  (`self.InitStateDelagate` (`self.CurrentState`))
  (if (`self.bDebug`)
    (`KismetSystemLibrary.PrintString` (`KismetStringLibrary.Concat_StrStr` (`KismetSystemLibrary.GetDisplayName` self) "" (`BlueprintGameplayTagLibrary.GetDebugStringFromGameplayTag` (`self.CurrentState`))) true true (struct :`R` 1.0 :`G` 0.3125 :`B` 0.998165 :`A` 1.0))))

(fn `IsCurrentState`
  (params (OtherContainer :type "GameplayTagContainer Structure (by ref)") (bExactMatch :type Boolean))
  (returns (AnyMatch :type Boolean))
  (return (`BlueprintGameplayTagLibrary.MatchesAnyTags` (`self.CurrentState`) OtherContainer bExactMatch)))

(fn `SwitchState`
  (params (NewState :type "GameplayTag Structure"))
  (returns (Successful :type Boolean))
  (if (and (!= NewState (struct)) (!= NewState (`self.CurrentState`)))
    (`self.EndState`)
    (set `self.CurrentState` NewState)
    (`self.InitState`)
    (set `self.CanTick` true)
    (`self.StateChanged`)
    (return true)
    (else
      (if (`self.bDebug`)
        (`KismetSystemLibrary.PrintString` "State Is Null or Already Active" true true (struct :`R` 1.0 :`B` 0.015156 :`A` 1.0) 4.0))
      (return false))))

(fn `TickState`
  (params (DeltaTime :type "Float (double-precision)"))
  (`self.TickStateDelagate` DeltaTime (`self.CurrentState`)))