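; BP_PickupSpawner is a placeable item pickup that adds its item to the interacting player's inventory.
; The construction script sizes a sphere from PickupRadius, then replaces any previous SpawnedItem with a new BP_ItemActor built from ItemTag.
; A successful AC_Interactable interaction passes that actor's item object to the controlled pawn's AC_Inventory, and the spawner destroys itself if the add succeeds.
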(event `self.AC_Interactable.OnInteractSuccess`
  (params (Instigator :type "Controller Object Reference"))
  (bind _spawneditem (`self.SpawnedItem`))
  (`/Engine/EditorBlueprintResources/StandardMacros.IsValid` _spawneditem
    (:`Is Valid`
      (bind _success (`/Game/InStudio/Blueprints/Components/AC_Inventory.AddItem` (`self.GetComponentByClass` (`Controller.K2_GetPawn` Instigator) "/Game/InStudio/Blueprints/Components/AC_Inventory.AC_Inventory_C") (`/Game/InStudio/Blueprints/Items/BP_ItemActor.Get Item Object` _spawneditem)))
      (if _success
        (`self.K2_DestroyActor`)))))

(fn `UpdateSpawnedItem`
  (bind _spawneditem (`self.SpawnedItem`))
  (`/Engine/EditorBlueprintResources/StandardMacros.IsValid` _spawneditem
    (:`Is Valid`
      (`self.K2_DestroyActor` _spawneditem))
    (:`Is Not Valid`
      _))
  (bind _returnvalue (`|SpawnActorFromClass` "/Game/InStudio/Blueprints/Items/BP_ItemActor.BP_ItemActor_C" (`self.GetTransform`) "Undefined" "MultiplyWithRoot" self (`self.ItemTag`) null))
  (set `self.SpawnedItem` _returnvalue))

(fn `UserConstructionScript`
  (`SphereComponent.SetSphereRadius` (`self.Sphere`) (`self.PickupRadius`) true)
  (`self.UpdateSpawnedItem`))