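; Saber weapon item actor that supplies the melee hit detection for its attack.
; TraceAttack sweeps a thin, tall box between the points from GetTraceStartEnd against pawns and destructibles, ignoring the owner and its child actors.
; The box takes its roll from the Reticle widget's render angle and its yaw from the owner, so the cut follows the reticle's tilt.
; It returns all hits and whether anything was struck.
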(fn `TraceAttack`
  (returns (HitResults :type "Array of HitResult Structure") (DidHit :type Boolean))
  (locals (IgnoreActors :type "Array of Actor Object Reference"))
  (bind _returnvalue (`self.GetOwner`))
  (bind (_returnvalue_roll _returnvalue_pitch _returnvalue_yaw) (`KismetMathLibrary.BreakRotator` (`self.K2_GetActorRotation` _returnvalue)))
  (bind _output_get (set `local.IgnoreActors` (`self.GetAllChildActors` _returnvalue true)))
  (`KismetArrayLibrary.Array_Add` _output_get _returnvalue)
  (bind (_startlocation _endlocation) (`self.Get Trace Start & End`))
  (bind (_outhits _returnvalue_2) (`KismetSystemLibrary.BoxTraceMultiForObjects` _startlocation _endlocation (1.0 1.0 30.0) (`KismetMathLibrary.MakeRotator` (`Widget.GetRenderTransformAngle` (`self.Reticle`)) 0.0 _returnvalue_yaw) (`|MakeArray` "ObjectTypeQuery3" "ObjectTypeQuery6" :!type "EObjectTypeQuery Enum") false (`local.IgnoreActors`)))
  (return _outhits _returnvalue_2))

(fn `UserConstructionScript`
  (`parent.UserConstructionScript`))