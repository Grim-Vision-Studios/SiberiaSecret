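; Single-leaf door child Blueprint that opens, closes or rattles its DoorLeft mesh in response to proximity and interaction.
; Overlapping DetectRange opens an unlocked door or rattles a locked one, and leaving the range closes it if unlocked.
; The ACInteractable component can activate only if the door is locked at construction.
; A successful interaction opens and unlocks the door, while a failed one rattles it.
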(event `self.ReceiveBeginPlay`
  (bind _ac_interactable (`self.AC_Interactable`))
  ;[1 1 1] Open Locked Door
  (add `/Game/InStudio/Blueprints/Components/AC_Interactable.OnInteracted` _ac_interactable (delegate `OnInteracted_Event`))
  ;[1 1 1] Rattle Door
  (add `/Game/InStudio/Blueprints/Components/AC_Interactable.OnFailedInteracted` _ac_interactable (delegate `OnFailedInteracted_Event`)))

(event `OnInteracted_Event`
  ;[1 1 1] Open Locked Door
  (`self.OpenDoor` (`self.Door_Left`) (stale `self.DetectRange.OnComponentBeginOverlap` OtherActor))
  (set `self.Locked` false))

(event `OnFailedInteracted_Event`
  ;[1 1 1] Rattle Door
  (`self.RattleDoor` (`self.Door_Left`) (stale `self.DetectRange.OnComponentBeginOverlap` OtherActor) :!label _label))

(event `self.DetectRange.OnComponentBeginOverlap`
  (params (OverlappedComponent :type "PrimitiveComponent Object Reference") (OtherActor :type "Actor Object Reference") (OtherComp :type "PrimitiveComponent Object Reference") (OtherBodyIndex :type Integer) (bFromSweep :type Boolean) (SweepResult :type "HitResult Structure (by ref)"))
  ;[1 1 1] Open Unlocked Door
  (if (`self.Locked`)
    (goto _label)
    (else
      (`self.OpenDoor` (`self.Door_Left`) OtherActor))))

(event `self.DetectRange.OnComponentEndOverlap`
  (params (OverlappedComponent :type "PrimitiveComponent Object Reference") (OtherActor :type "Actor Object Reference") (OtherComp :type "PrimitiveComponent Object Reference") (OtherBodyIndex :type Integer))
  ;[1 1 1] Close Door
  (if (not (`self.Locked`))
    (`self.CloseDoor`)))

(fn `UserConstructionScript`
  (set `self.TargetMesh` (`self.Door_Left`))
  (`parent.UserConstructionScript`)
  (set `/Game/InStudio/Blueprints/Components/AC_Interactable.CanActivate` (`self.Locked`) (`self.AC_Interactable`)))