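; BP_Door_Core is a door actor with open, close and locked-rattle events, apparently a base for specific door types.
; Timelines drive the yaw of the passed-in mesh for a reversible swing or a short rattle, signed by IsActorOnPosY for the interacting actor.
; Rattling also sends a locked message to the HUD.
; The construction script sizes the detection sphere and picks one of three wooden door meshes from DoorType.
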(event `OpenDoor`
  (params (RotateMesh :type "StaticMeshComponent Object Reference") (OtherActor :type "Actor Object Reference"))
  (if (not (`self.IsOpen`))
    (set `self.NegY` (`self.IsActorOnPosY` OtherActor))
    (set `self.IsOpen` true)
    ;[1 1 1] Open & Close Door
    (bind (_direction _rotationcoeff) (`Timeline|Timeline_Rotation` :!label _label)
      (:`Update`
        (bind _returnvalue (* _rotationcoeff 92.0))
        (`SceneComponent.K2_SetRelativeRotation` RotateMesh (`KismetMathLibrary.MakeRotator` 0.0 0.0 (`KismetMathLibrary.SelectFloat` _returnvalue (* _returnvalue -1.0) (`self.NegY`))) false false)))))

(event `CloseDoor`
  (if (`self.IsOpen`)
    (set `self.IsOpen` false)
    (goto _label :!via `Reverse`)))

(event `RattleDoor`
  (params (RattleMesh :type "StaticMeshComponent Object Reference") (OtherActor :type "Actor Object Reference"))
  (set `self.NegY` (`self.IsActorOnPosY` OtherActor))
  (message `/Game/InStudio/Blueprints/Interfaces/I_Hud.SendNotification` (`PlayerController.GetHUD` (`GameplayStatics.GetPlayerController` 0)) (`self.LockedMessage`) (`self.MessageDisplayTime`))
  ;[1 1 1] Rattle Locked Door
  (bind (_direction _rotationcoeff) (`Timeline|Timeline` :!via `PlayFromStart`)
    (:`Update`
      (bind _returnvalue (* _rotationcoeff 6.0))
      (`SceneComponent.K2_SetRelativeRotation` RattleMesh (`KismetMathLibrary.MakeRotator` 0.0 0.0 (`KismetMathLibrary.SelectFloat` _returnvalue (* _returnvalue -1.0) (`self.NegY`))) false false))))

(fn `UserConstructionScript`
  (bind _targetmesh (`self.TargetMesh`))
  (`SphereComponent.SetSphereRadius` (`self.DetectRange`) (`self.DetectionRadius`) true)
  (bind _output_get (set `self.DoorType` (`KismetMathLibrary.Clamp` (`self.DoorType`) 0 2)))
  (switch `int` _output_get
    (:`0`
      (`StaticMeshComponent.SetStaticMesh` _targetmesh "/Game/Medieval_Environment/Medieval_Houses_Vol2/Meshes/SM_MH_02_Wood_Door_01.SM_MH_02_Wood_Door_01"))
    (:`1`
      (`StaticMeshComponent.SetStaticMesh` _targetmesh "/Game/Medieval_Environment/Medieval_Houses_Vol2/Meshes/SM_MH_02_Wood_Door_02.SM_MH_02_Wood_Door_02"))
    (:`2`
      (`StaticMeshComponent.SetStaticMesh` _targetmesh "/Game/Medieval_Environment/Medieval_Houses_Vol2/Meshes/SM_MH_02_Wood_Door_03.SM_MH_02_Wood_Door_03"))))