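; Actor component that tracks which interactable its owner is currently overlapping.
; It binds to the owner's begin and end overlap events and looks for an AC_Interactable component on the other actor.
; The newest one found becomes the single current interactable, cleared only when its own overlap ends.
; Changes fire found and lost dispatchers, and GetInteractable exposes the current target with a validity flag.
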(event `self.ReceiveBeginPlay`
  ;[1 1 1] Show Interactable
  (add `Actor.OnActorBeginOverlap` (`self.GetOwner`) (delegate `CheckOverlapForInteractable`))
  ;[1 1 1] Forget Interactable
  (add `Actor.OnActorEndOverlap` (`self.GetOwner`) (delegate `ForgetInteractabe`)))

(event `ForgetInteractabe`
  (params (OverlappedActor :type "Actor Object Reference") (OtherActor :type "Actor Object Reference"))
  (bind _returnvalue (`Actor.GetComponentByClass` OtherActor "/Game/InStudio/Blueprints/Systems/Interact/AC_Interactable.AC_Interactable_C"))
  ;[1 1 1] Forget Interactable
  (`/Engine/EditorBlueprintResources/StandardMacros.IsValid` _returnvalue
    (:`Is Valid`
      (if (== _returnvalue (`self.CurrentInteractable`))
        (`self.SetInteractable` null)))))

(event `CheckOverlapForInteractable`
  (params (OverlappedActor :type "Actor Object Reference") (OtherActor :type "Actor Object Reference"))
  (bind _returnvalue (`Actor.GetComponentByClass` OtherActor "/Game/InStudio/Blueprints/Systems/Interact/AC_Interactable.AC_Interactable_C"))
  ;[1 1 1] Show Interactable
  (`/Engine/EditorBlueprintResources/StandardMacros.IsValid` _returnvalue
    (:`Is Valid`
      (`self.SetInteractable` _returnvalue))))

(event `SetInteractable`
  (params (CurrentInteractable :type "/Game/InStudio/Blueprints/Systems/Interact/AC_Interactable Object Reference"))
  (`/Engine/EditorBlueprintResources/StandardMacros.IsValid` CurrentInteractable
    (:`Is Valid`
      (bind _output_get (set `self.CurrentInteractable` CurrentInteractable))
      (`self.OnInteractFound` _output_get))
    (:`Is Not Valid`
      (`self.OnInteractLost` (`self.CurrentInteractable`))
      (set `self.CurrentInteractable` null))))

(fn `GetInteractable`
  (returns (IsValid :type Boolean) (CurrentInteractable :type "/Game/InStudio/Blueprints/Systems/Interact/AC_Interactable Object Reference"))
  (bind _currentinteractable (`self.CurrentInteractable`))
  (return (`KismetSystemLibrary.IsValid` _currentinteractable) _currentinteractable))