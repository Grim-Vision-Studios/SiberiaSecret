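; AC_Interactable is an actor component that lets its owner be interacted with and tracks whether it is in use.
; On BeginPlay it caches the owner's AC_InteractWidget, which SetShowInteract uses to show or hide the interact message.
; Interact fires OnInteracted with the instigator only while not in use, and SetInUse stores the flag and broadcasts OnInUseSet.
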(event `self.ReceiveBeginPlay`
  (bind _returnvalue (`Actor.GetComponentByClass` (`self.GetOwner`) "/Game/InStudio/Blueprints/Systems/Interact/AC_InteractWidget.AC_InteractWidget_C"))
  (`/Engine/EditorBlueprintResources/StandardMacros.IsValid` _returnvalue
    (:`Is Valid`
      (set `self.InteractWidget` _returnvalue))))

(event `Interact`
  (params (Instigator :type "Controller Object Reference"))
  (if (not (`self.InUse`))
    (`self.OnInteracted` Instigator)))

(event `SetShowInteract`
  (params (ShowInteract :type Boolean))
  (bind _interactwidget (`self.InteractWidget`))
  (if ShowInteract
    (`/Game/InStudio/Blueprints/Systems/Interact/AC_InteractWidget.ShowInteractMessage` _interactwidget)
    (else
      (`/Game/InStudio/Blueprints/Systems/Interact/AC_InteractWidget.HideInteractMessage` _interactwidget))))

(event `SetInUse`
  (params (`In Use` :type Boolean))
  (bind _output_get (set `self.InUse` `In Use`))
  (`self.OnInUseSet` _output_get))

(fn `GetInUse`
  (returns (IsUsed :type Boolean))
  (return (`self.InUse`)))