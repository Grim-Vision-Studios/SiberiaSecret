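; Widget component that shows and hides an interaction message in the game.
; On BeginPlay it caches its widget as a W_InteractMessage.
; Show and hide events play that widget's ShowInteract animation forward or in reverse, with an IsShown flag preventing repeat triggers.
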(event `self.ReceiveBeginPlay`
  (bind _asw_interact_message (cast `/Game/InStudio/Art/UI/W_InteractMessage` (`self.GetWidget`)))
  (set `self.InteractMessageWidget` _asw_interact_message))

(event `ShowInteractMessage`
  (bind _interactmessagewidget (`self.InteractMessageWidget`))
  (if (not (`self.IsShown`))
    (set `self.IsShown` true)
    (`UserWidget.PlayAnimation` _interactmessagewidget (`/Game/InStudio/Art/UI/W_InteractMessage.ShowInteract` _interactmessagewidget) 0.0 1 "Forward" 1.0 false)))

(event `HideInteractMessage`
  (bind _interactmessagewidget (`self.InteractMessageWidget`))
  (if (`self.IsShown`)
    (set `self.IsShown` false)
    (`UserWidget.PlayAnimation` _interactmessagewidget (`/Game/InStudio/Art/UI/W_InteractMessage.ShowInteract` _interactmessagewidget) 0.0 1 "Reverse" 1.0 false)))