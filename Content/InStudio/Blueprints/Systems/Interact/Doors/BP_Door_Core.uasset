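; Core interactable door that swings open, closes, or rattles when locked, with a choice of three wooden door meshes set at construction.
; Interact extends the parent's interaction and uses its response to toggle the door or play the rattle.
; Timelines drive the mesh's yaw, flipping its sign by the instigator's side, with closing reversing the open timeline.
; Finishing either timeline clears the in-use state.
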(event `OpenDoor`
  (params (Instigator :type "Actor Object Reference"))
  (if (not (`self.IsOpen`))
    (set `self.NegY` (`self.IsActorOnPosY` Instigator))
    (set `self.IsOpen` true)
    ;[1 1 1] Open & Close Door
    (bind (_direction _rotationcoeff) (`Timeline|Timeline_OpenClose` :!label _label)
      (:`Update`
        (bind _returnvalue (* _rotationcoeff 92.0))
        (`SceneComponent.K2_SetRelativeRotation` (`self.TargetMesh`) (`KismetMathLibrary.MakeRotator` 0.0 0.0 (`KismetMathLibrary.SelectFloat` _returnvalue (* _returnvalue -1.0) (`self.NegY`))) false false))
      (:`Finished`
        (`self.SetInUse` false)))))

(event `CloseDoor`
  (if (`self.IsOpen`)
    (set `self.IsOpen` false)
    (goto _label :!via `Reverse`)))

(event `RattleDoor`
  (params (Instigator :type "Actor Object Reference"))
  (set `self.NegY` (`self.IsActorOnPosY` Instigator))
  ;[1 1 1] Rattle Locked Door
  (bind (_direction _rotationcoeff) (`Timeline|Timeline_Rattle` :!via `PlayFromStart`)
    (:`Update`
      (bind _returnvalue (* _rotationcoeff 6.0))
      (`SceneComponent.K2_SetRelativeRotation` (`self.TargetMesh`) (`KismetMathLibrary.MakeRotator` 0.0 0.0 (`KismetMathLibrary.SelectFloat` _returnvalue (* _returnvalue -1.0) (`self.NegY`))) false false))
    (:`Finished`
      (`self.SetInUse` false))))

(fn `Interact`
  (params (Instigator :type "Controller Object Reference"))
  (returns (Response :type "/Game/InStudio/Blueprints/Data/Enums/E_InteractResponse Enum"))
  (locals (CurrentResponse :type "/Game/InStudio/Blueprints/Data/Enums/E_InteractResponse Enum" :default "NewEnumerator2"))
  (bind _response (`parent.Interact` Instigator))
  (bind _output_get (set `local.CurrentResponse` _response))
  (switch `/Game/InStudio/Blueprints/Data/Enums/E_InteractResponse` _output_get
    (:`NewEnumerator2`
      (if (`self.IsOpen`)
        (`self.CloseDoor`)
        (else
          (`self.OpenDoor` (`local.Instigator`)))))
    (:`NewEnumerator0`
      _)
    (:`NewEnumerator1`
      (`self.RattleDoor` (`local.Instigator`))))
  (return (`local.CurrentResponse`)))

(fn `UserConstructionScript`
  (bind _targetmesh (`self.TargetMesh`))
  (set `self.Detect Collision` (`self.GetDetectCollision`))
  (bind _output_get (set `self.DoorType` (`KismetMathLibrary.Clamp` (`self.DoorType`) 0 2)))
  (switch `int` _output_get
    (:`0`
      (`StaticMeshComponent.SetStaticMesh` _targetmesh "/Game/Medieval_Environment/Medieval_Houses_Vol2/Meshes/SM_MH_02_Wood_Door_01.SM_MH_02_Wood_Door_01"))
    (:`1`
      (`StaticMeshComponent.SetStaticMesh` _targetmesh "/Game/Medieval_Environment/Medieval_Houses_Vol2/Meshes/SM_MH_02_Wood_Door_02.SM_MH_02_Wood_Door_02"))
    (:`2`
      (`StaticMeshComponent.SetStaticMesh` _targetmesh "/Game/Medieval_Environment/Medieval_Houses_Vol2/Meshes/SM_MH_02_Wood_Door_03.SM_MH_02_Wood_Door_03"))))