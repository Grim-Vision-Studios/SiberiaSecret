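; BP_Interactable is a base interactable actor that shows a prompt on overlap and manages locked and in-use states.
; Empty getters, apparently meant for child overrides, supply the detection collision and widget, whose overlap events show or hide the message without filtering actors.
; Interact returns an enum result: locked sends a HUD notification, busy is rejected, otherwise it sets InUse and fires OnInUseSet.
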(event `self.ReceiveBeginPlay`
  (bind _detect_collision (`self.GetDetectCollision`))
  (add `PrimitiveComponent.OnComponentBeginOverlap` _detect_collision (delegate `DetectBeginOverlap`))
  (add `PrimitiveComponent.OnComponentEndOverlap` _detect_collision (delegate `DetectEndOverlap`))
  (set `self.InteractWidget` (`self.GetInteractWidget`)))

(event `DetectBeginOverlap`
  (params (OverlappedComponent :type "PrimitiveComponent Object Reference") (OtherActor :type "Actor Object Reference") (OtherComp :type "PrimitiveComponent Object Reference") (OtherBodyIndex :type Integer) (bFromSweep :type Boolean) (SweepResult :type "HitResult Structure (by ref)"))
  (`self.SetShowInteract` true))

(event `DetectEndOverlap`
  (params (OverlappedComponent :type "PrimitiveComponent Object Reference") (OtherActor :type "Actor Object Reference") (OtherComp :type "PrimitiveComponent Object Reference") (OtherBodyIndex :type Integer))
  (`self.SetShowInteract` false))

(event `SetShowInteract`
  (params (ShowInteract :type Boolean))
  (bind _interactwidget (`self.InteractWidget`))
  (if ShowInteract
    (`/Game/InStudio/Blueprints/Systems/Interact/AC_InteractWidget.ShowInteractMessage` _interactwidget)
    (else
      (`/Game/InStudio/Blueprints/Systems/Interact/AC_InteractWidget.HideInteractMessage` _interactwidget))))

(fn `GetDetectCollision`
  (returns (`Detect Collision` :type "PrimitiveComponent Object Reference"))
  (return null))

(fn `GetInteractWidget`
  (returns (InteractWidget :type "/Game/InStudio/Blueprints/Systems/Interact/AC_InteractWidget Object Reference"))
  (return null))

(fn `GetInUse`
  (returns (`In Use` :type Boolean))
  (return (`self.In Use`)))

(fn `GetLocked`
  (returns (Locked :type Boolean))
  (return (`self.Locked`)))

(fn `Interact`
  (params (Instigator :type "Controller Object Reference"))
  (returns (Response :type "/Game/InStudio/Blueprints/Data/Enums/E_InteractResponse Enum"))
  (if (`self.GetLocked`)
    (message `/Game/InStudio/Blueprints/Interfaces/I_Notif.SendNotification` (`PlayerController.GetHUD` (`GameplayStatics.GetPlayerController` 0)) (`self.LockedMessage`) (`self.LockedMessageTime`))
    (return "NewEnumerator1")
    (elif (`self.GetInUse`)
      (return "NewEnumerator0")
      (else
        (`self.SetInUse` true)
        (return "NewEnumerator2")))))

(fn `SetInUse`
  (params (`In Use` :type Boolean))
  (bind _output_get (set `self.In Use` `In Use`))
  (`self.OnInUseSet` _output_get))

(fn `UserConstructionScript`)