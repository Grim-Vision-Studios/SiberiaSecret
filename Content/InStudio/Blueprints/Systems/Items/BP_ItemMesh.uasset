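; BP_ItemMesh is an item actor that assembles its visual from several static mesh components in the Construction Script.
; Each MeshToSpawn key is a source component whose mesh and relative transform are copied into a new component, stored in SpawnedMeshes.
; The map's value is a parent index, attaching that copy to an earlier one to rebuild the hierarchy.
; Copies have no collision, are hidden from their owner and cast hidden shadows.
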(event `self.ReceiveBeginPlay`)

(fn `UserConstructionScript`
  (locals (SpawnedMeshes :type "Array of StaticMeshComponent Object Reference") (CurrentIndex :type Integer))
  (bind _meshtospawn (`self.MeshToSpawn`))
  (bind _keys (`BlueprintMapLibrary.Map_Keys` _meshtospawn))
  (for (_array_element _array_index) _keys
    (set `local.CurrentIndex` _array_index)
    (`|ExecutionSequence`
      (:`then_0`
        (bind _returnvalue (`AddComponent|NODE_AddStaticMeshComponent-0` :`RelativeTransform` (`SceneComponent.GetRelativeTransform` _array_element)))
        (`KismetArrayLibrary.Array_Set` (`local.SpawnedMeshes`) (`local.CurrentIndex`) _returnvalue true)
        (`StaticMeshComponent.SetStaticMesh` _returnvalue (`StaticMeshComponent.StaticMesh` _array_element))
        (`PrimitiveComponent.SetOwnerNoSee` _returnvalue true)
        (`PrimitiveComponent.SetCollisionEnabled` _returnvalue "NoCollision")
        (`PrimitiveComponent.SetCastHiddenShadow` _returnvalue true))
      (:`then_1`
        (bind _value (`BlueprintMapLibrary.Map_Find` _meshtospawn _array_element))
        (if (>= _value 0)
          (bind _output (`|GetArrayItem` (`local.SpawnedMeshes`) _value))
          (`/Engine/EditorBlueprintResources/StandardMacros.IsValid` _output
            (:`Is Valid`
              (`SceneComponent.K2_AttachToComponent` _returnvalue _output "None" "KeepRelative" "KeepRelative" "KeepRelative" true))))))))