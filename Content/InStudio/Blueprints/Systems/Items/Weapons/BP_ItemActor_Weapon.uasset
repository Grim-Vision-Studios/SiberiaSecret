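; Base weapon item actor that aims through a screen reticle and applies point damage to traced targets.
; PrepareItem enables per-tick TraceAttack, a stub returning no hit, whose results tint the reticle and get cached.
; UseItem stops tracing, damages cached hits and returns the owner to Idle.
; Helpers deproject the reticle center for trace endpoints, show owner-only meshes and spawn mesh actors, while upgrade functions are empty.
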(event `self.ReceiveBeginPlay`
  (bind _returnvalue (`|CreateWidget` (`self.ReticleClass`) (`GameplayStatics.GetPlayerController` 0)))
  (set `self.Reticle` _returnvalue))

(event `self.ReceiveTick`
  (params (DeltaSeconds :type "Float (single-precision)"))
  (if (`self.Trace`)
    (bind (_hitresults _didhit) (`self.TraceAttack`))
    (if _didhit
      (if (`KismetArrayLibrary.Array_IsEmpty` (`self.LastHitResults`))
        (`self.SetReticleSight` true)
        (set `self.LastHitResults` _hitresults))
      (else
        (`self.SetReticleSight` false)
        (`KismetArrayLibrary.Array_Clear` (`self.LastHitResults`))))))

(fn `ApplayUpgrades`)

(fn `Damage Last Traced Actors`
  (bind _lasthitresults (`self.LastHitResults`))
  (if (`KismetArrayLibrary.Array_IsNotEmpty` _lasthitresults)
    (for _array_element _lasthitresults
      (bind (_bblockinghit _binitialoverlap _time _distance _location _impactpoint _normal _impactnormal _physmat _hitactor) (`GameplayStatics.BreakHitResult` _array_element))
      (`GameplayStatics.ApplyPointDamage` _hitactor (`.Damage_34_D92E50E843155C6427C1EC8B8C7E705A` (break `/Game/InStudio/Blueprints/Data/Stucts/S_WeaponStats` (`self.WeaponStats`))) _impactnormal _array_element (`GameplayStatics.GetPlayerController` 0) (`self.GetOwner`)))))

(fn `Get Trace Start & End`
  (returns (StartLocation :type "Vector Structure") (EndLocation :type "Vector Structure"))
  (bind _returnvalue (`Widget.GetCachedGeometry` (`self.Reticle`)))
  (bind (_worldposition _worlddirection) (`GameplayStatics.DeprojectScreenToWorld` (`GameplayStatics.GetPlayerController` 0) (`SlateBlueprintLibrary.LocalToViewport` _returnvalue (/ (`SlateBlueprintLibrary.GetLocalSize` _returnvalue) (2.0 2.0)))))
  (return _worldposition (+ _worldposition (* _worlddirection (`.Range_45_C1B2003443182BBF98F705A9AB9B9E27` (break `/Game/InStudio/Blueprints/Data/Stucts/S_WeaponStats` (`self.WeaponStats`)))))))

(fn `PrepareItem`
  (set `self.Trace` true))

(fn `Reveal to Owner`
  (bind _weapontop (`self.WeaponTop`))
  (`PrimitiveComponent.SetOwnerNoSee` _weapontop false)
  (`PrimitiveComponent.SetOwnerNoSee` (`self.BaseMesh`) false)
  (`PrimitiveComponent.SetOnlyOwnerSee` _weapontop true)
  (`PrimitiveComponent.SetOnlyOwnerSee` (`self.BaseMesh`) true)
  (`PrimitiveComponent.SetCastShadow` _weapontop false)
  (`PrimitiveComponent.SetCastShadow` (`self.BaseMesh`) false))

(fn `SetReticleSight`
  (params (NewSight :type Boolean))
  (locals (InSightColor :type "LinearColor Structure" :default (struct :`R` 1.0 :`G` 0.255208 :`B` 0.255208 :`A` 1.0)) (OutOfSightColor :type "LinearColor Structure" :default (struct :`R` 1.0 :`G` 1.0 :`B` 1.0 :`A` 1.0)))
  (`UserWidget.SetColorAndOpacity` (`self.Reticle`) (`KismetMathLibrary.SelectColor` (`local.InSightColor`) (`local.OutOfSightColor`) NewSight)))

(fn `SpawnMeshActor`
  (returns (MeshActor :type "/Game/InStudio/Blueprints/Systems/Items/BP_ItemMesh Object Reference"))
  (bind _returnvalue (`|SpawnActorFromClass` "/Game/InStudio/Blueprints/Systems/Items/BP_ItemMesh.BP_ItemMesh_C" (`self.GetTransform`) "Undefined" "MultiplyWithRoot" (`self.GetOwner`) (`|MakeMap` (`self.BaseMesh`) -1 (`self.WeaponTop`)) null))
  (return _returnvalue))

(fn `TraceAttack`
  (returns (HitResults :type "Array of HitResult Structure") (DidHit :type Boolean))
  (return _ false))

(fn `UpgradeStatWithTag`
  (params (StatTag :type Name) (UpgradeValue :type Integer)))

(fn `UseItem`
  (set `self.Trace` false)
  (`self.Damage Last Traced Actors`)
  (message `/Game/InStudio/Blueprints/Interfaces/I_StateMachine.SwitchState` (`self.GetOwner`) (struct :`TagName` "Actions.Idle"))
  (return))

(fn `UserConstructionScript`
  (`self.ApplayUpgrades`))