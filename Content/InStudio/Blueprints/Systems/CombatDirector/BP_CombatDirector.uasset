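; Combat director that takes turns granting one enemy permission to attack through the "CanAttack?" Blackboard key.
; A looping timer clears that key across EnemyList and gives each enemy with "PlayerSpotted?" set a random score in the EnemyGrading map.
; FindHighest picks the top-scored enemy to enable, and a Delay re-runs the selection alongside the timer to reshuffle scores.
; EnemyList is not populated within this Blueprint.
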(event `self.ReceiveBeginPlay`
  (`KismetSystemLibrary.K2_SetTimerDelegate` (delegate `Loop`) 3.0 true))

(event `Loop`
  (for _array_element (`self.EnemyList`) :!label _label
    (`BlackboardComponent.SetValueAsBool` (`AIBlueprintHelperLibrary.GetBlackboard` _array_element) "CanAttack?" false)
    (`/Engine/EditorBlueprintResources/StandardMacros.IsValid` _array_element
      (:`Is Valid`
        (if (`BlackboardComponent.GetValueAsBool` (`AIBlueprintHelperLibrary.GetBlackboard` _array_element) "PlayerSpotted?")
          (`BlueprintMapLibrary.Map_Add` (`self.EnemyGrading`) _array_element (`KismetMathLibrary.RandomFloatInRange` 1.0 5.0))))))
  (bind _loc_highestratedenemy1 (`self.FindHighest`))
  (`/Engine/EditorBlueprintResources/StandardMacros.IsValid` _loc_highestratedenemy1
    (:`Is Valid`
      (`BlackboardComponent.SetValueAsBool` (`AIBlueprintHelperLibrary.GetBlackboard` _loc_highestratedenemy1) "CanAttack?" true)
      ;[1 1 1] Go back and change all enemies numbers once cycled through
      (`KismetSystemLibrary.Delay` 5.0)
      (goto _label))))

(fn `FindHighest`
  (returns (Loc_HighestRatedEnemy1 :type "/Game/InStudio/Blueprints/Entities/BP_Entity_Base Object Reference"))
  (locals (Loc_HighestValue :type "Float (double-precision)") (Loc_HighestRatedEnemy :type "/Game/InStudio/Blueprints/Entities/BP_Entity_Base Object Reference"))
  (for _array_element (`self.EnemyList`)
    (bind _value (`BlueprintMapLibrary.Map_Find` (`self.EnemyGrading`) _array_element))
    (if (> _value (`local.Loc_HighestValue`))
      (set `local.Loc_HighestValue` _value)
      (set `local.Loc_HighestRatedEnemy` _array_element)
      (else
        (`BlackboardComponent.SetValueAsBool` (`AIBlueprintHelperLibrary.GetBlackboard` _array_element) "CanAttack?" false))))
  (return (`local.Loc_HighestRatedEnemy`)))

(fn `UserConstructionScript`)