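; Behavior tree task for the Strygza AI that records where the player is and how far away they are from the controlled pawn.
; On execute it takes player character 0 and writes its location and its distance to the pawn into two blackboard keys.
; It samples once per execution, finishing with success, or with failure when no valid player character exists.
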(event `self.ReceiveExecuteAI`
  (params (OwnerController :type "AIController Object Reference") (ControlledPawn :type "Pawn Object Reference"))
  (bind _returnvalue (`GameplayStatics.GetPlayerCharacter` 0))
  (bind _returnvalue_2 (`Actor.K2_GetActorLocation` _returnvalue))
  (`/Engine/EditorBlueprintResources/StandardMacros.IsValid` _returnvalue
    (:`Is Valid`
      (`BTFunctionLibrary.SetBlackboardValueAsVector` (`self.PlayerLocation`) _returnvalue_2)
      (`BTFunctionLibrary.SetBlackboardValueAsFloat` (`self.DistanceToPlayer`) (`KismetMathLibrary.Vector_Distance` _returnvalue_2 (`Actor.K2_GetActorLocation` ControlledPawn)))
      (`self.FinishExecute` true))
    (:`Is Not Valid`
      (`self.FinishExecute` false))))