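; BP_Entity_Strygza is the Blueprint for the Strygza entity, feeding player detection and random values into its AI Blackboard.
; On BeginPlay it binds CreateInt to a RandomInt event, and CreateInt writes a small random integer to the "Int" key.
; When the player character enters the PlayerDetection component, it sets "PlayerSpotted?" to true, with no reset in this graph.
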(event `self.ReceiveBeginPlay`
  (add `self.RandomInt` (delegate `CreateInt`)))

(event `CreateInt`
  (`BlackboardComponent.SetValueAsInt` (`AIBlueprintHelperLibrary.GetBlackboard` null) (`self.Int`) (`KismetMathLibrary.RandomIntegerInRange` 1 3)))

(event `self.PlayerDetection.OnComponentBeginOverlap`
  (params (OverlappedComponent :type "PrimitiveComponent Object Reference") (OtherActor :type "Actor Object Reference") (OtherComp :type "PrimitiveComponent Object Reference") (OtherBodyIndex :type Integer) (bFromSweep :type Boolean) (SweepResult :type "HitResult Structure (by ref)"))
  (if (== (`GameplayStatics.GetPlayerCharacter` 0) OtherActor)
    (`BlackboardComponent.SetValueAsBool` (`AIBlueprintHelperLibrary.GetBlackboard` null) "PlayerSpotted?" true)))

(fn `UserConstructionScript`)