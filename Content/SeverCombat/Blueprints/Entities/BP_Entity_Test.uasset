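; BP_Entity_Test is a test entity in SeverCombat whose construction script classifies its body part components.
; After running the parent script, it finds BPC_BodyPart components tagged Torso, Head or Limb and sets each one's BodyPartType, taking only the first Torso.
; Disconnected, unfinished nodes hold an approach that reads a data table, maps rows into BodyHealth and updates skeletal meshes.
; BeginPlay is empty.
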(event `self.ReceiveBeginPlay`)

(fn `UserConstructionScript`
  (locals (CurrentBodyPartData :type "/Game/SeverCombat/Blueprints/Data/S_BodyPart Structure") (CurrentComponent :type "/Game/SeverCombat/Blueprints/BPC_BodyPart Object Reference"))
  (`parent.UserConstructionScript`)
  (`|ExecutionSequence`
    (:`then_0`
      (set `local.CurrentComponent` (`|GetArrayItem` (`self.GetComponentsByTag` "/Game/SeverCombat/Blueprints/BPC_BodyPart.BPC_BodyPart_C" "Torso")))
      (set `/Game/SeverCombat/Blueprints/BPC_BodyPart.BodyPartType` "NewEnumerator2" (`local.CurrentComponent`)))
    (:`then_1`
      (for _array_element (`self.GetComponentsByTag` "/Game/SeverCombat/Blueprints/BPC_BodyPart.BPC_BodyPart_C" "Head")
        (set `local.CurrentComponent` _array_element)
        (set `/Game/SeverCombat/Blueprints/BPC_BodyPart.BodyPartType` "NewEnumerator0" (`local.CurrentComponent`))))
    (:`then_2`
      (for _array_element_2 (`self.GetComponentsByTag` "/Game/SeverCombat/Blueprints/BPC_BodyPart.BPC_BodyPart_C" "Limb")
        (set `local.CurrentComponent` _array_element_2)
        (set `/Game/SeverCombat/Blueprints/BPC_BodyPart.BodyPartType` "NewEnumerator1" (`local.CurrentComponent`))))))