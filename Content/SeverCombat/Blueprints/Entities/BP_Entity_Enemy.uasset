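; Modular enemy entity for SeverCombat, built from separate head and limb meshes that follow CoreMesh's pose from BeginPlay.
; The construction script loads EntityTable rows, maps tagged mesh components to them by body-part type in BodyHealth, then applies each mapped mesh.
; The torso type check is unwired, so that pass maps nothing.
; The limb loop sets CurrentBodyPart to None instead of the row before its type check.
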(event `self.ReceiveBeginPlay`
  (`SkinnedMeshComponent.SetLeaderPoseComponent` (`self.Head`) (`self.CoreMesh`) false)
  (`SkinnedMeshComponent.SetLeaderPoseComponent` (`self.RArm`) (`self.CoreMesh`) false)
  (`SkinnedMeshComponent.SetLeaderPoseComponent` (`self.LArm`) (`self.CoreMesh`) false)
  (`SkinnedMeshComponent.SetLeaderPoseComponent` (`self.LLeg`) (`self.CoreMesh`) false)
  (`SkinnedMeshComponent.SetLeaderPoseComponent` (`self.RLeg`) (`self.CoreMesh`) false))

(fn `UserConstructionScript`
  (locals (CurrentComponent :type "SkeletalMeshComponent Object Reference") (CurrentBodyPart :type "/Game/SeverCombat/Blueprints/Data/S_BodyPart Structure"))
  (bind _bodyparts (`/Game/SeverCombat/Blueprints/BP_BodyHealth.BodyParts` (`self.BodyHealth`)))
  (`parent.UserConstructionScript`)
  (`|ExecutionSequence`
    (:`then_0`
      ;[1 1 1] Get body part data from Data Table
      (bind _outrownames (`DataTableFunctionLibrary.GetDataTableRowNames` (`self.Entity Table`)))
      (for _array_element _outrownames
        (bind _returnvalue (`|GetDataTableRow` (`self.Entity Table`) _array_element)
          (:`then`
            (`KismetArrayLibrary.Array_AddUnique` (`self.BodyPartData`) _returnvalue)))))
    (:`then_1`
      ;[1 1 1] Map Body Data with skeletal mesh key
      (bind _asskeletal_mesh_component (cast `SkeletalMeshComponent` (`|GetArrayItem` (`self.GetComponentsByTag` "/Script/Engine.ActorComponent" "Torso"))))
      (set `local.CurrentComponent` _asskeletal_mesh_component)
      (for _array_element_2 (`self.BodyPartData`)
        (bind _output_get (set `local.CurrentBodyPart` _array_element_2))))
    (:`then_2`
      (for _array_element_3 (`self.GetComponentsByTag` "/Script/Engine.ActorComponent" "Head")
        (bind _asskeletal_mesh_component_2 (cast `SkeletalMeshComponent` _array_element_3))
        (set `local.CurrentComponent` _asskeletal_mesh_component_2)
        (for _array_element_4 (`self.BodyPartData`)
          (bind _output_get_2 (set `local.CurrentBodyPart` _array_element_4))
          (if (`|EnumEquality` (`.BodyPartType_14_B252B0794059528096A444ABF2E970FC` (break `/Game/SeverCombat/Blueprints/Data/S_BodyPart` _output_get_2)) "NewEnumerator0")
            (`BlueprintMapLibrary.Map_Add` (`/Game/SeverCombat/Blueprints/BP_BodyHealth.BodyParts` (`self.BodyHealth`)) (`local.CurrentComponent`) (`local.CurrentBodyPart`) :!label _label)))))
    (:`then_3`
      (for _array_element_5 (`self.GetComponentsByTag` "/Script/Engine.ActorComponent" "Limb")
        (bind _asskeletal_mesh_component_3 (cast `SkeletalMeshComponent` _array_element_5))
        (set `local.CurrentComponent` _asskeletal_mesh_component_3)
        (for _ (`self.BodyPartData`)
          (bind _output_get_3 (set `local.CurrentBodyPart` (struct)))
          (if (`|EnumEquality` (`.BodyPartType_14_B252B0794059528096A444ABF2E970FC` (break `/Game/SeverCombat/Blueprints/Data/S_BodyPart` _output_get_3)) "NewEnumerator1")
            (goto _label))))
      ;[1 1 1] Update Bod Meshes
      (bind _keys (`BlueprintMapLibrary.Map_Keys` _bodyparts))
      (for _array_element_6 _keys
        (`SkinnedMeshComponent.SetSkinnedAssetAndUpdate` _array_element_6 (`.Mesh_11_2843BAA74EE097D6469CF4A71AAAEDE1` (break `/Game/SeverCombat/Blueprints/Data/S_BodyPart` (`BlueprintMapLibrary.Map_Find` _bodyparts _array_element_6))) true)))))